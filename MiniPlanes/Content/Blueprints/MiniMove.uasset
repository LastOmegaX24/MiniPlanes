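; GMC movement component for BP_MiniAircraft that flies it toward the point under the player's cursor.
; It loads stats from a data table by aircraft name, while thrust input adjusts a clamped target speed.
; Each prediction tick traces the cursor, yaws by a speed-based curve, bleeds speed in turns, moves forward and turns the cone cosmetically.
; Inputs and movement state are bound for replication, mixing client and server authority.
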(event `self.ReceiveBeginPlay`
  (bind _asbp_mini_aircraft (cast `/Game/Blueprints/BP_MiniAircraft` (`self.GetGMCPawnOwner`)))
  (bind _output_get (set `self.As BP Mini Aircraft` _asbp_mini_aircraft))
  (bind _returnvalue (`|GetDataTableRow` (`self.StatDataTable`) (`/Game/Blueprints/BP_MiniAircraft.AircraftName` _output_get))
    (:`then`
      (set `self.AircraftData` _returnvalue)
      (bind _asgmc_player_controller (cast `GMC_PlayerController` (`GameplayStatics.GetPlayerControllerFromID` 0)))
      (set `self.As GMC Player Controller` _asgmc_player_controller)
      (`EnhancedInputSubsystemInterface.AddMappingContext` (pcsubsystem `EnhancedInputLocalPlayerSubsystem` _asgmc_player_controller) "/Game/Input/KBM.KBM" 0 (struct)))))

(event `self.GenPredictionTick`
  (params (DeltaTime :type "Float (single-precision)"))
  (`self.ClientHittrace`)
  (`self.RotateToPointer`)
  (`self.TurnSlow`)
  (`self.Move` DeltaTime)
  (`self.CosmeticTurn`))

(event `ClientHittrace`
  (bind _as_gmc_player_controller (`self.As GMC Player Controller`))
  (bind (_bblockinghit _binitialoverlap _time _distance _location _impactpoint) (`GameplayStatics.BreakHitResult` (`PlayerController.GetHitResultUnderCursorForObjects` _as_gmc_player_controller (`|MakeArray` "ObjectTypeQuery1" :!type "EObjectTypeQuery Enum") false)))
  (`/Engine/EditorBlueprintResources/StandardMacros.IsValid` _as_gmc_player_controller
    (:`Is Valid`
      (if _bblockinghit
        (set `self.Impact Point` _impactpoint)))))

(event `self.BindReplicationData`
  (`parent.BindReplicationData`)
  (`self.BindDoublePrecisionFloat` (`self.TargetThrust`) "ClientAuth_Input" "CombineIfUnchanged" "Periodic_Output" "NearestNeighbour")
  (`self.BindCompressedVector` (`self.Impact Point`) "ClientAuth_Input" "AlwaysCombine" "PeriodicAndOnChange_Output" "NearestNeighbour")
  (`self.BindDoublePrecisionFloat` (`self.MaxThrust`) "ServerAuth_InputOutput_ServerValidated" "AlwaysCombine" "Periodic_Output" "NearestNeighbour")
  (`self.BindActorReference` (`self.As GMC Player Controller`) "ClientAuth_Input" "AlwaysCombine" "Periodic_Output" "NearestNeighbour")
  (`self.BindDoublePrecisionFloat` (`self.CurrentSpeed`) "ServerAuth_InputOutput_ServerValidated" "AlwaysCombine" "Periodic_Output" "NearestNeighbour")
  (`self.BindCompressedRotator` (`self.TargetRot`) "ClientAuth_Input" "AlwaysCombine" "None" "NearestNeighbour")
  (`self.BindCompressedRotator` (`self.CurrentRot`) "ServerAuth_Output_ClientValidated" "CombineIfUnchanged" "Periodic_InputOutput" "NearestNeighbour"))

(event `EnhancedInput|/Game/Input/Thrust`
  (params (ActionValue :type "Float (double-precision)") (ElapsedSeconds :type "Float (double-precision)") (TriggeredSeconds :type "Float (double-precision)") (InputAction :type "InputAction Object Reference" :default "/Game/Input/Thrust.Thrust"))
  (bind (_maxthrust _maxspeed _minspeedstall) (break `/Game/AircraftData/AircraftDataStructure` (`self.AircraftData`)))
  (:`Triggered`
    (set `self.TargetThrust` (`KismetMathLibrary.FClamp` (+ (`self.TargetThrust`) (* (`self.ThrustSens`) (`self.GetPhysDeltaTime`) ActionValue)) _minspeedstall _maxthrust) :!label _label))
  (:`Ongoing`
    (goto _label)))

(fn `CosmeticTurn`
  (`SceneComponent.K2_SetRelativeRotation` (`/Game/Blueprints/BP_MiniAircraft.Cone` (`self.As BP Mini Aircraft`)) (`KismetMathLibrary.MakeRotator` 0.0 (- (.yaw (`self.TargetRot`)) (.yaw (`self.GetRootCollisionRotation`)))) false false))

(fn `Move`
  (params (DeltaTime :type "Float (single-precision)"))
  (bind (_aircraftdata_maxthrust _aircraftdata_maxspeed _aircraftdata_minspeedstall _aircraftdata_reservemissiles _aircraftdata_turnspeed _aircraftdata_acceleration) (break `/Game/AircraftData/AircraftDataStructure` (`self.AircraftData`)))
  (set `self.CurrentSpeed` (`KismetMathLibrary.FInterpTo_Constant` (`self.CurrentSpeed`) (`self.TargetThrust`) DeltaTime _aircraftdata_acceleration))
  (`self.UpdateVelocity` (* (`self.CurrentSpeed`) (`Actor.GetActorForwardVector` (`self.GetGMCPawnOwner`))) DeltaTime)
  (`self.K2_MoveUpdatedComponent` (* (`self.GetVelocity`) DeltaTime) (`self.GetRootCollisionRotation`)))

(fn `RotateToPointer`
  (bind _output_get (set `self.TargetRot` (`KismetMathLibrary.FindLookAtRotation` (`self.GetRootCollisionLocation`) (`self.Impact Point`))))
  (bind _output_get_2 (set `self.CurrentRot` (`KismetMathLibrary.MakeRotator` 0.0 0.0 (.yaw (`KismetMathLibrary.RLerp` (`self.GetRootCollisionRotation`) _output_get (`CurveFloat.GetFloatValue` (`.Turnspeed_17_FF247B81499497AE758C9C960762844A` (break `/Game/AircraftData/AircraftDataStructure` (`self.AircraftData`))) (`self.CurrentSpeed`)) true)))))
  (`Actor.K2_SetActorRotation` (`self.GetPawnOwner`) _output_get_2 false))

(fn `TurnSlow`
  (set `self.CurrentSpeed` (- (`self.CurrentSpeed`) (`CurveFloat.GetFloatValue` (`.RateSpeed_24_176D276F417AE96FF01A18B9DE8B46F6` (break `/Game/AircraftData/AircraftDataStructure` (`self.AircraftData`))) (`KismetMathLibrary.Abs` (/ (- (.yaw (`self.TargetRot`)) (.yaw (`self.GetRootCollisionRotation`))) 180.0))))))