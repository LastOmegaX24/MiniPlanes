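; Game mode that handles player respawns, map travel and ready-state refresh for an aircraft game.
; Respawn calls go through an RPC event that, on authority, spawns a BP_Spectator carrying the plane class, spawn transform and initial-spawn flag, then has the controller possess it.
; Map changes run a ServerTravel console command with the listen option.
; Ready refreshes unload and reload every 3D_MenuPawn with the ReadyPlayers data.
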(event `/Game/Blueprints/Interface/RespawnPlayer.RespawnCall`
  (params (Controller :type "PlayerController Object Reference") (Transform :type "Transform Structure") (Aircraft :type "/Game/Blueprints/BP_MiniAircraft Class Reference") (Initial :type Boolean))
  (`self.RPC_RespawnCall` Controller Transform Aircraft Initial))

(event `RPC_RespawnCall`
  (params (NewParam :type "PlayerController Object Reference") (NewParam2 :type "Transform Structure") (PlaneClass :type "/Game/Blueprints/BP_MiniAircraft Class Reference") (InitialSpawn :type Boolean))
  (`/Engine/EditorBlueprintResources/StandardMacros.IsValid` NewParam
    (:`Is Valid`
      (`/Engine/EditorBlueprintResources/ActorMacros.Switch Has Authority`
        (:`Authority`
          (bind _returnvalue (`|SpawnActorFromClass` "/Game/Blueprints/BP_Spectator.BP_Spectator_C" NewParam2 "AlwaysSpawn" "MultiplyWithRoot" null InitialSpawn NewParam2 PlaneClass null))
          (`Controller.Possess` NewParam _returnvalue))))))

(event `OpenLevel`
  (params (MapStruct :type "/Game/MapData/MapStruct Structure (by ref)"))
  (`KismetSystemLibrary.ExecuteConsoleCommand` (`KismetStringLibrary.Concat_StrStr` "ServerTravel " (`.MapName_5_9404071F448FE89004A3B2872BA4A78A` (break `/Game/MapData/MapStruct` MapStruct)) "?Listen") null))

(event `RefreshAllPlayerReady`
  (`self.RPC_RefreshAll`))

(event `RPC_RefreshAll`
  (bind _outactors (`GameplayStatics.GetAllActorsOfClass` "/Game/Blueprints/System/3D_MenuPawn.3D_MenuPawn_C"))
  (for _array_element _outactors
    (`/Game/Blueprints/System/3D_MenuPawn.Unload` _array_element)
    (`/Game/Blueprints/System/3D_MenuPawn.Load` _array_element (`self.ReadyPlayers`))))

(fn `UserConstructionScript`)