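; Target-lock indicator actor that attaches to a target and displays lock-on progress through a Target_Lock_Prog widget.
; Each tick it copies LockProgression to the widget, first draining it over time when not locking, and looks up its parent's index in the player's AlreadyTrackingProg.
; LoseLockDelay holds IsLocking true through a retriggerable two-second delay.
; The actor destroys itself when its attach parent or PlayerRef becomes invalid.
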(event `self.ReceiveBeginPlay`
  (bind _astarget_lock_prog (cast `/Game/HUD/Target_Lock_Prog` (`WidgetComponent.GetWidget` (`self.Widget`))))
  (set `self.As Lock Prog Widget` _astarget_lock_prog))

(event `LoseLockDelay`
  (set `self.IsLocking` true)
  (`KismetSystemLibrary.RetriggerableDelay` 2.0)
  (set `self.IsLocking` false))

(event `self.ReceiveTick`
  (params (DeltaSeconds :type "Float (single-precision)"))
  (bind _returnvalue (`self.GetAttachParentActor`))
  (bind _playerref (`self.PlayerRef`))
  (`/Engine/EditorBlueprintResources/StandardMacros.IsValid` _returnvalue
    (:`Is Valid`
      (`/Engine/EditorBlueprintResources/StandardMacros.IsValid` _playerref
        (:`Is Valid`
          (set `self.CurrentTargetIndex` (`KismetArrayLibrary.Array_Find` (`/Game/Blueprints/BP_MiniAircraft.AlreadyTrackingProg` _playerref) _returnvalue))
          (if (`self.IsLocking`)
            (set `/Game/HUD/Target_Lock_Prog.Progress` (`self.LockProgression`) (`self.As Lock Prog Widget`))
            (else
              (set `self.LockProgression` (- (`self.LockProgression`) (* DeltaSeconds 3.0)))
              (set `/Game/HUD/Target_Lock_Prog.Progress` (`self.LockProgression`) (`self.As Lock Prog Widget`)))))
        (:`Is Not Valid`
          (`self.K2_DestroyActor` :!label _label))))
    (:`Is Not Valid`
      (goto _label))))

(fn `OnRep_LockProgression`)

(fn `UserConstructionScript`)