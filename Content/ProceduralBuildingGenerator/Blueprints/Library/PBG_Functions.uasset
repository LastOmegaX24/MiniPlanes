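; Blueprint function library for the Procedural Building Generator, providing mesh measurement, spline editing and small geometry helpers.
; Mesh sizes come from "dim" or per-axis sockets, tolerating misspelled names, with orientation-aware bounds as fallback.
; Spline helpers copy, transform, retype, rebuild without aligned points, and fix winding by reversing points when the shoelace signed area is negative.
; Other helpers generate rotated box corners, random name tags and 2D vector arrays.
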(fn `PBG Auto Correct Spline Orientation`
  (params (`Spline Ref` :type "SplineComponent Object Reference"))
  (locals (RPoints :type "Array of Vector Structure"))
  (if (> (`SplineComponent.GetNumberOfSplinePoints` `Spline Ref`) 2)
    (bind _points (`self.PBG Get Spline Points` (`local.Spline Ref`)))
    (bind _output_get (set `local.RPoints` _points))
    (bind _signed_area (`self.PBG Calculate Polygon Area` _output_get))
    (if (< _signed_area 0.0)
      (`KismetArrayLibrary.Array_Reverse` (`local.RPoints`))
      (`SplineComponent.SetSplinePoints` (`local.Spline Ref`) (`local.RPoints`) "World" true))))

(fn `PBG Calculate Polygon Area`
  (params (Vertices :type "Array of Vector Structure"))
  (returns (`Signed Area` :type "Float (double-precision)") (`Is Valid` :type Boolean))
  (locals (NVertices :type "Array of Vector Structure") (`Max Loop` :type Integer) (`Total Area` :type "Float (double-precision)") (NIndex :type Integer))
  (bind _nvertices (`local.NVertices`))
  (bind (_output_x _output_y) (`KismetMathLibrary.BreakVector` (`|GetArrayItem` (`local.NVertices`) (`local.NIndex`))))
  (bind _returnvalue (/ (`local.Total Area`) 2.0))
  (bind (_output_x_2 _output_y_2) (`KismetMathLibrary.BreakVector` (`|GetArrayItem` (`local.NVertices`) (+ (`local.NIndex`) 1))))
  (set `local.NVertices` Vertices)
  (set `local.Max Loop` (- (`KismetArrayLibrary.Array_Length` Vertices) 1))
  (`KismetArrayLibrary.Array_Add` _nvertices (`|GetArrayItem` _nvertices))
  (for _index (range (+ (`local.Max Loop`) 1))
    (set `local.NIndex` _index)
    (set `local.Total Area` (+ (`local.Total Area`) (- (* _output_x _output_y_2) (* _output_y _output_x_2)))))
  (return _returnvalue (not (`KismetMathLibrary.NearlyEqual_FloatFloat` _returnvalue))))

(fn `PBG Create Spline From Points`
  (params (Spline :type "SplineComponent Object Reference") (Points :type "Array of Vector Structure") (CoordinateSpace :type "ESplineCoordinateSpace Enum" :default "Local"))
  (`SplineComponent.SetSplinePoints` Spline Points CoordinateSpace true))

(fn `PBG Create Spline From Spline`
  (params (`Source Spline` :type "SplineComponent Object Reference") (`Target Spline` :type "SplineComponent Object Reference (by ref)") (`Spline Height` :type "Float (double-precision)") (`Use Custom Spline Height` :type Boolean :default true))
  (locals (`Spline ` :type "SplineComponent Object Reference") (Vertices :type "Array of Vector Structure") (Index :type Integer) (`Point Type` :type "Array of ESplinePointType Enum"))
  (bind (_returnvalue_x _returnvalue_y _returnvalue_z) (`KismetMathLibrary.BreakVector` (`SplineComponent.GetLocationAtSplinePoint` (`local.Spline `) (`local.Index`) "World")))
  (set `local.Spline ` `Source Spline`)
  (for _index (range (`SplineComponent.GetNumberOfSplinePoints` (`local.Spline `)))
    (set `local.Index` _index)
    (`KismetArrayLibrary.Array_Add` (`local.Vertices`) (`KismetMathLibrary.MakeVector` _returnvalue_x _returnvalue_y (select `bool` `Use Custom Spline Height` :`false` _returnvalue_z :`true` `Spline Height`)))
    (`KismetArrayLibrary.Array_Add` (`local.Point Type`) (`SplineComponent.GetSplinePointType` (`local.Spline `) (`local.Index`))))
  (`SplineComponent.ClearSplinePoints` `Target Spline` true)
  (`SplineComponent.SetSplinePoints` `Target Spline` (`local.Vertices`) "World" true)
  (for _index_2 (range (`SplineComponent.GetNumberOfSplinePoints` `Target Spline`))
    (set `local.Index` _index_2)
    (`SplineComponent.SetSplinePointType` `Target Spline` (`local.Index`) (`|GetArrayItem` (`local.Point Type`) (`local.Index`)) true)))

(fn `PBG Get Points From Box With Rotation`
  (params (`Box Origin ` :type "Vector Structure") (`Scaled Box Extent` :type "Vector Structure") (`Z Rotation` :type "Float (single-precision)"))
  (returns (Points :type "Array of Vector Structure"))
  (locals (`Box Origin   ` :type "Vector Structure"))
  (bind (_returnvalue_x _returnvalue_y) (`KismetMathLibrary.BreakVector` (* `Scaled Box Extent` 1)))
  (bind (_returnvalue_x_2 _returnvalue_y_2) (`KismetMathLibrary.BreakVector` (* `Scaled Box Extent` -1)))
  (bind _box_origin___ (`local.Box Origin   `))
  (set `local.Box Origin   ` `Box Origin `)
  (return (`|MakeArray` (`KismetMathLibrary.TransformLocation` (`KismetMathLibrary.MakeTransform` _box_origin___ (`KismetMathLibrary.MakeRotator` 0.0 0.0 `Z Rotation`)) (`KismetMathLibrary.MakeVector` _returnvalue_x _returnvalue_y_2)) (`KismetMathLibrary.TransformLocation` (`KismetMathLibrary.MakeTransform` _box_origin___ (`KismetMathLibrary.MakeRotator` 0.0 0.0 `Z Rotation`)) (`KismetMathLibrary.MakeVector` _returnvalue_x _returnvalue_y)) (`KismetMathLibrary.TransformLocation` (`KismetMathLibrary.MakeTransform` _box_origin___ (`KismetMathLibrary.MakeRotator` 0.0 0.0 `Z Rotation`)) (`KismetMathLibrary.MakeVector` _returnvalue_x_2 _returnvalue_y)) (`KismetMathLibrary.TransformLocation` (`KismetMathLibrary.MakeTransform` _box_origin___ (`KismetMathLibrary.MakeRotator` 0.0 0.0 `Z Rotation`)) (`KismetMathLibrary.MakeVector` _returnvalue_x_2 _returnvalue_y_2)))))

(fn `PBG Get Spline Points`
  (params (Spline :type "SplineComponent Object Reference") (CoordinateSpace :type "ESplineCoordinateSpace Enum" :default "World") (`Add Location` :type "Vector Structure"))
  (returns (Points :type "Array of Vector Structure") (`Tangents ` :type "Array of Vector Structure"))
  (locals (`Points   ` :type "Array of Vector Structure") (Tangents :type "Array of Vector Structure"))
  (for _index (range (`SplineComponent.GetNumberOfSplinePoints` Spline))
    (`KismetArrayLibrary.Array_Add` (`local.Points   `) (+ (`SplineComponent.GetLocationAtSplinePoint` Spline _index CoordinateSpace) (`local.Add Location`)))
    (`KismetArrayLibrary.Array_Add` (`local.Tangents`) (`SplineComponent.GetTangentAtSplinePoint` Spline _index CoordinateSpace)))
  (return (`local.Points   `) (`local.Tangents`)))

(fn `PBG Random Tag`
  (params (`Pre String` :type String :default "PCC") (`End String` :type String :default "Gen"))
  (returns (`Random Tag` :type Name))
  (locals (Letters :type "Array of String"))
  (bind _outitem (`KismetArrayLibrary.Array_Random` (`local.Letters`)))
  (return (`KismetStringLibrary.Conv_StringToName` (`KismetStringLibrary.Concat_StrStr` (`KismetStringLibrary.Concat_StrStr` `Pre String` "_") (`KismetStringLibrary.Conv_IntToString` (`KismetMathLibrary.RandomInteger` 7000000)) (select `bool` (`KismetMathLibrary.RandomBool`) :`false` (`KismetStringLibrary.Concat_StrStr` _outitem `End String` "_") :`true` (`KismetStringLibrary.Concat_StrStr` "_" `End String` _outitem)) (`KismetStringLibrary.Conv_IntToString` (`KismetMathLibrary.RandomInteger` 700000)) (`KismetStringLibrary.Concat_StrStr` "_" (`KismetStringLibrary.Conv_IntToString` (`KismetMathLibrary.RandomInteger` 1000)) (`KismetArrayLibrary.Array_Random` (`local.Letters`)) (`KismetStringLibrary.Conv_IntToString` (`KismetMathLibrary.RandomInteger` 1000)))))))

(fn `PBG Remove Aligned Points`
  (params (`Spline Ref` :type "SplineComponent Object Reference (by ref)") (`Error Tolerance ` :type "Float (single-precision)" :default 0.0001) (`Keep Linear` :type Boolean :default true))
  (locals (`Spline Ref ` :type "SplineComponent Object Reference") (`Direction ` :type "Vector Structure") (`Error Tolerance` :type "Float (single-precision)" :default 0.0001) (Index :type Integer) (`Previous Direction` :type "Vector Structure") (`Number Of Points` :type Integer) (`Points To Remove` :type "Array of Integer") (`All Points` :type "Array of Integer") (`Non Aligned Points` :type "Array of Vector Structure"))
  (bind _returnvalue (`SplineComponent.GetNumberOfSplinePoints` (`local.Spline Ref `)))
  (set `local.Spline Ref ` `Spline Ref`)
  (set `local.Error Tolerance` `Error Tolerance `)
  (if (> _returnvalue 2)
    (set `local.Number Of Points` (- _returnvalue 1))
    (set `local.Previous Direction` (`SplineComponent.GetDirectionAtSplinePoint` (`local.Spline Ref `) (`local.Number Of Points`) "Local"))
    ;[1 1 1] Loop to search for points that have same direction! store them
    (for _index (range (+ (`local.Number Of Points`) 1))
      (bind _output_get (set `local.Index` _index))
      (bind _output_get_2 (set `local.Direction ` (`SplineComponent.GetDirectionAtSplinePoint` (`local.Spline Ref `) _output_get "Local")))
      (if (== _output_get_2 (`local.Previous Direction`) :`ErrorTolerance` (`local.Error Tolerance`))
        (`KismetArrayLibrary.Array_Add` (`local.Points To Remove`) (`local.Index`)))
      (set `local.Previous Direction` (`local.Direction `))
      (`KismetArrayLibrary.Array_Add` (`local.All Points`) (`local.Index`)))
    ;[1 1 1] Remove Aligned Points ID
    (for _array_element (`local.Points To Remove`)
      (if (`KismetArrayLibrary.Array_Contains` (`local.All Points`) _array_element)
        (`KismetArrayLibrary.Array_RemoveItem` (`local.All Points`) _array_element)))
    ;[1 1 1] Store Non Aligned Points Location
    (for _array_element_2 (`local.All Points`)
      (`KismetArrayLibrary.Array_Add` (`local.Non Aligned Points`) (`SplineComponent.GetLocationAtSplinePoint` (`local.Spline Ref `) _array_element_2 "Local")))
    ;[1 1 1] Reconstruct Spline using non aligned Points
    (`SplineComponent.ClearSplinePoints` (`local.Spline Ref `) true)
    (`SplineComponent.SetSplinePoints` (`local.Spline Ref `) (`local.Non Aligned Points`) "Local" true)
    (if `Keep Linear`
      (`self.PBG Set All Point Types` (`local.Spline Ref `)))))

(fn `PBG Set All Point Types`
  (params (`Spline Ref` :type "SplineComponent Object Reference (by ref)") (Type :type "ESplinePointType Enum" :default "Linear"))
  (locals (`Spline Ref ` :type "SplineComponent Object Reference") (Distance :type "Float (double-precision)") (Radius :type "Float (single-precision)" :default 1.0) (Index :type Integer) (`Previous Distance` :type "Float (double-precision)" :default 2.0) (`Number Of Points` :type Integer) (`Points To Remove` :type "Array of Integer") (`All Points` :type "Array of Integer") (`Non Closest Points` :type "Array of Vector Structure"))
  (`/Engine/EditorBlueprintResources/StandardMacros.IsValid` `Spline Ref`
    (:`Is Valid`
      (for _index (range (`SplineComponent.GetNumberOfSplinePoints` `Spline Ref`))
        (`SplineComponent.SetSplinePointType` `Spline Ref` _index Type true)))))

(fn `PBG Transform Spline`
  (params (`Spline Ref` :type "SplineComponent Object Reference (by ref)") (Transform :type "Transform Structure"))
  (locals (`Spline Ref ` :type "SplineComponent Object Reference") (Distance :type "Float (double-precision)") (Radius :type "Float (single-precision)" :default 1.0) (Index :type Integer) (`Previous Distance` :type "Float (double-precision)" :default 2.0) (`Number Of Points` :type Integer) (`Points To Remove` :type "Array of Integer") (`All Points` :type "Array of Integer") (`Non Closest Points` :type "Array of Vector Structure"))
  (`SceneComponent.K2_AddLocalTransform` `Spline Ref` Transform false false))

(fn `PBG Vectors to 2D`
  (params (Points :type "Array of Vector Structure"))
  (returns (`2D Points` :type "Array of Vector2D Structure"))
  (locals (`2Ds` :type "Array of Vector2D Structure"))
  (for _array_element Points
    (`KismetArrayLibrary.Array_Add` (`local.2Ds`) (`KismetMathLibrary.Conv_VectorToVector2D` _array_element)))
  (return (`local.2Ds`)))

(fn `PBG_Calculate Static Mesh Size`
  (params (`Static Meshe` :type "StaticMesh Object Reference") (`Mesh Orientation` :type "/Game/ProceduralBuildingGenerator/Blueprints/PBG_Data/PBG_Axis_Orientation Enum" :default "NewEnumerator8"))
  (returns (`Mesh X size` :type "Float (double-precision)") (`Mesh Y size` :type "Float (double-precision)") (`Mesh Z size` :type "Float (double-precision)") (`Static Mesh` :type "StaticMesh Object Reference"))
  (bind (_depth _length_ _height _valid_depth__ _valid_length _valid_height__) (`self.PBG_Get Size By Socket_FC` (`local.Static Meshe`)))
  (bind (_returnvalue_origin _returnvalue_boxextent) (`KismetMathLibrary.BreakBoxSphereBounds` (`StaticMesh.GetBounds` (`local.Static Meshe`))))
  (bind _x (.x (* _returnvalue_boxextent 2)))
  (bind _y (.y (* _returnvalue_boxextent 2)))
  (`/Engine/EditorBlueprintResources/StandardMacros.IsValid` `Static Meshe`
    (:`Is Valid`
      (return (select `bool` _valid_depth__ :`false` (select `/Game/ProceduralBuildingGenerator/Blueprints/PBG_Data/PBG_Axis_Orientation` (`local.Mesh Orientation`) :`NewEnumerator8` _x :`NewEnumerator9` _y) :`true` _depth) (select `bool` _valid_length :`false` (select `/Game/ProceduralBuildingGenerator/Blueprints/PBG_Data/PBG_Axis_Orientation` (`local.Mesh Orientation`) :`NewEnumerator8` _y :`NewEnumerator9` _x) :`true` _length_) (select `bool` _valid_height__ :`false` (.z (* _returnvalue_boxextent 2)) :`true` _height) (`local.Static Meshe`)))
    (:`Is Not Valid`
      (return 0.0 0.0 0.0 null))))

(fn `PBG_Calculate Static Mesh Size_FC`
  (params (`Static Mesh ` :type "StaticMesh Object Reference") (`Mesh Orientation` :type "/Game/ProceduralBuildingGenerator/Blueprints/PBG_Data/PBG_Axis_Orientation Enum" :default "NewEnumerator8"))
  (returns (`Mesh X size` :type "Float (double-precision)") (`Mesh Y size` :type "Float (double-precision)") (`Mesh Z size` :type "Float (double-precision)") (`Static Mesh` :type "StaticMesh Object Reference"))
  (bind (_depth _length_ _height _valid_depth__ _valid_length _valid_height__) (`self.PBG_Get Size By Socket_FC` `Static Mesh `))
  (bind (_returnvalue_origin _returnvalue_boxextent) (`KismetMathLibrary.BreakBoxSphereBounds` (`StaticMesh.GetBounds` `Static Mesh `)))
  (bind _x (.x (* _returnvalue_boxextent 2)))
  (bind _y (.y (* _returnvalue_boxextent 2)))
  (`/Engine/EditorBlueprintResources/StandardMacros.IsValid` `Static Mesh `
    (:`Is Valid`
      (return (select `bool` _valid_depth__ :`false` (select `/Game/ProceduralBuildingGenerator/Blueprints/PBG_Data/PBG_Axis_Orientation` (`local.Mesh Orientation`) :`NewEnumerator8` _x :`NewEnumerator9` _y) :`true` _depth) (select `bool` _valid_length :`false` (select `/Game/ProceduralBuildingGenerator/Blueprints/PBG_Data/PBG_Axis_Orientation` (`local.Mesh Orientation`) :`NewEnumerator8` _y :`NewEnumerator9` _x) :`true` _length_) (select `bool` _valid_height__ :`false` (.z (* _returnvalue_boxextent 2)) :`true` _height) `Static Mesh `))
    (:`Is Not Valid`
      (return 0.0 0.0 0.0 null))))

(fn `PBG_Get Size By Socket_FC`
  (params (Mesh :type "StaticMesh Object Reference"))
  (returns (Depth :type "Float (double-precision)") (`Length ` :type "Float (double-precision)") (Height :type "Float (double-precision)") (`Valid Depth  ` :type Boolean) (`Valid Length` :type Boolean) (`Valid Height  ` :type Boolean))
  (locals (`Valid Lenght` :type Boolean) (`Valid Height` :type Boolean) (`Valid Depth` :type Boolean) (Heigth :type "Float (double-precision)") (Length :type "Float (double-precision)") (`Depth ` :type "Float (double-precision)"))
  (bind _returnvalue (`StaticMesh.FindSocket` Mesh "dim"))
  (bind _relativelocation_x (`KismetMathLibrary.BreakVector` (`StaticMeshSocket.RelativeLocation` (`StaticMesh.FindSocket` Mesh "depht"))))
  (bind (_relativelocation_x_2 _relativelocation_y _relativelocation_z) (`KismetMathLibrary.BreakVector` (`StaticMeshSocket.RelativeLocation` (`StaticMesh.FindSocket` Mesh "heigth"))))
  (bind (_relativelocation_x_3 _relativelocation_y_2) (`KismetMathLibrary.BreakVector` (`StaticMeshSocket.RelativeLocation` (`StaticMesh.FindSocket` Mesh "length"))))
  (bind (_relativelocation_x_4 _relativelocation_y_3 _relativelocation_z_2) (`KismetMathLibrary.BreakVector` (`StaticMeshSocket.RelativeLocation` _returnvalue)))
  (bind _relativelocation_x_5 (`KismetMathLibrary.BreakVector` (`StaticMeshSocket.RelativeLocation` (`StaticMesh.FindSocket` Mesh "depth"))))
  (bind (_relativelocation_x_6 _relativelocation_y_4) (`KismetMathLibrary.BreakVector` (`StaticMeshSocket.RelativeLocation` (`StaticMesh.FindSocket` Mesh "lenght"))))
  (bind (_relativelocation_x_7 _relativelocation_y_5 _relativelocation_z_3) (`KismetMathLibrary.BreakVector` (`StaticMeshSocket.RelativeLocation` (`StaticMesh.FindSocket` Mesh "height"))))
  (`/Engine/EditorBlueprintResources/StandardMacros.IsValid` Mesh
    (:`Is Valid`
      (`/Engine/EditorBlueprintResources/StandardMacros.IsValid` _returnvalue
        (:`Is Valid`
          (set `local.Depth ` (`KismetMathLibrary.Abs` _relativelocation_x_4))
          (set `local.Length` (`KismetMathLibrary.Abs` _relativelocation_y_3))
          (set `local.Heigth` (`KismetMathLibrary.Abs` _relativelocation_z_2))
          (set `local.Valid Lenght` true)
          (set `local.Valid Height` true)
          (set `local.Valid Depth` true)
          (return (`local.Depth `) (`local.Length`) (`local.Heigth`) (`local.Valid Depth`) (`local.Valid Lenght`) (`local.Valid Height`)))
        (:`Is Not Valid`
          (`|ExecutionSequence`
            (:`then_0`
              (`/Engine/EditorBlueprintResources/StandardMacros.IsValid` (`StaticMesh.FindSocket` Mesh "depth")
                (:`Is Valid`
                  (set `local.Valid Depth` true)
                  (set `local.Depth ` (`KismetMathLibrary.Abs` _relativelocation_x_5)))
                (:`Is Not Valid`
                  (`/Engine/EditorBlueprintResources/StandardMacros.IsValid` (`StaticMesh.FindSocket` Mesh "depht")
                    (:`Is Valid`
                      (set `local.Valid Depth` true)
                      (set `local.Depth ` (`KismetMathLibrary.Abs` _relativelocation_x)))
                    (:`Is Not Valid`
                      (set `local.Valid Depth` false))))))
            (:`then_1`
              (`/Engine/EditorBlueprintResources/StandardMacros.IsValid` (`StaticMesh.FindSocket` Mesh "height")
                (:`Is Valid`
                  (set `local.Valid Height` true)
                  (set `local.Heigth` (`KismetMathLibrary.Abs` _relativelocation_z_3)))
                (:`Is Not Valid`
                  (`/Engine/EditorBlueprintResources/StandardMacros.IsValid` (`StaticMesh.FindSocket` Mesh "heigth")
                    (:`Is Valid`
                      (set `local.Valid Height` true)
                      (set `local.Heigth` (`KismetMathLibrary.Abs` _relativelocation_z)))
                    (:`Is Not Valid`
                      (set `local.Valid Height` false))))))
            (:`then_2`
              (`/Engine/EditorBlueprintResources/StandardMacros.IsValid` (`StaticMesh.FindSocket` Mesh "lenght")
                (:`Is Valid`
                  (set `local.Valid Lenght` true)
                  (set `local.Length` (`KismetMathLibrary.Abs` _relativelocation_y_4)))
                (:`Is Not Valid`
                  (`/Engine/EditorBlueprintResources/StandardMacros.IsValid` (`StaticMesh.FindSocket` Mesh "length")
                    (:`Is Valid`
                      (set `local.Valid Lenght` true)
                      (set `local.Length` (`KismetMathLibrary.Abs` _relativelocation_y_2)))
                    (:`Is Not Valid`
                      (set `local.Valid Lenght` false))))))
            (:`then_3`
              (return (`local.Depth `) (`local.Length`) (`local.Heigth`) (`local.Valid Depth`) (`local.Valid Lenght`) (`local.Valid Height`)))))))
    (:`Is Not Valid`
      (return 0.0 0.0 0.0 false false false))))