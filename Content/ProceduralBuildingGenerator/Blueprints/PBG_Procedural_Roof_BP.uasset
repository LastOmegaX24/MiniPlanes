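; Procedural roof actor for the building generator that fills a polygon outline with a flat Geometry Script mesh.
; Construction optionally refreshes the vertices from an orientation-corrected spline; mesh rebuilds triangulate them in 2D, raise the result to roof height and can flip normals.
; A bake function saves the mesh as a Nanite static mesh with complex collision, spawns it with the actor's tags minus the optimization tag, then destroys the generator.
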(event `self.OnRebuildGeneratedMesh`
  (params (TargetMesh :type "DynamicMesh Object Reference"))
  (`self.Create Shape`))

(fn `Bake Mesh To Content Browser`
  (locals (`Mesh Ref` :type "StaticMesh Object Reference"))
  (bind _returnvalue (`EditorAssetLibrary.DoesDirectoryExist` (`self.Asset Path`)))
  (if _returnvalue
    (`self.Create Shape`)
    (bind _returnvalue_2 (`BaseDynamicMeshComponent.GetDynamicMesh` (`self.DynamicMeshComponent`)))
    (bind _returnvalue_3 (`GeometryScriptLibrary_CreateNewAssetFunctions.CreateNewStaticMeshAssetFromMesh` _returnvalue_2 (`KismetStringLibrary.Concat_StrStr` (`self.Asset Path`) (`KismetStringLibrary.Conv_NameToString` (`/Game/ProceduralBuildingGenerator/Blueprints/Library/PBG_Functions.PBG Random Tag` "Roof" "Baked"))) (make `GeometryScriptCreateNewStaticMeshAssetOptions` false false true (make `MeshNaniteSettings` true) 0.0 true "CTF_UseComplexAsSimple") null)
      (:`Failure`
        (`KismetSystemLibrary.PrintString` "Unable to bake mesh; make sure you created a folder labeled \"PBG_Baked\" in the content browser" true true (struct :`R` 1.0 :`A` 1.0) 15.0))
      (:`Success`
        (bind _output_get (set `local.Mesh Ref` _returnvalue_3))
        (`GeometryScriptLibrary_CollisionFunctions.SetStaticMeshCollisionFromComponent` _output_get (`self.DynamicMeshComponent`) (struct :`bEmitTransaction` true) null)
        (`StaticMesh.SetMaterial` (`local.Mesh Ref`) 0 (`self.Material`))
        ;[1 1 1] Remove opti Z tag
        (`KismetArrayLibrary.Array_RemoveItem` (`self.Tags`) (`self.OptiZ Tag`))
        (bind _returnvalue_4 (`EditorLevelLibrary.SpawnActorFromObject` (`local.Mesh Ref`) (`self.K2_GetActorLocation`) (`self.Roof Rotation`)))
        (set `Actor.Tags` (`self.Tags`) _returnvalue_4)
        (`KismetSystemLibrary.PrintString` "Sucessfully baked mesh in the \"PBG_Baked\" folder" true true (struct :`G` 1.0 :`A` 1.0) 3.5)
        (`self.K2_DestroyActor`)))
    (else
      (`KismetSystemLibrary.PrintString` "Unable to bake mesh; make sure you created a folder labeled \"PBG_Baked\" in the content browser" true true (struct :`R` 1.0 :`A` 1.0) 15.0))))

(fn `Create Shape`
  (locals (`Polygon Vertices` :type "Array of Vector2D Structure"))
  (bind (_roof_location_x _roof_location_y _roof_location_z) (`KismetMathLibrary.BreakVector` (`self.Roof Location`)))
  (bind _returnvalue (`BaseDynamicMeshComponent.GetDynamicMesh` (`self.DynamicMeshComponent`)))
  (`DynamicMesh.Reset` _returnvalue)
  (if (>= (`KismetArrayLibrary.Array_Length` (`self.Vertex`)) 3)
    (for _array_element (`self.Vertex`)
      (`KismetArrayLibrary.Array_Add` (`local.Polygon Vertices`) (`KismetMathLibrary.Conv_VectorToVector2D` _array_element)))
    (bind _returnvalue_2 (`BaseDynamicMeshComponent.GetDynamicMesh` (`self.DynamicMeshComponent`)))
    (`GeometryScriptLibrary_MeshPrimitiveFunctions.AppendTriangulatedPolygon` _returnvalue_2 (make `GeometryScriptPrimitiveOptions` "PerFace" false "ScaleToFill") (struct) (`local.Polygon Vertices`) true null)
    (`PrimitiveComponent.SetMaterial` (`self.DynamicMeshComponent`) 0 (`self.Material`))
    (bind _returnvalue_3 (`BaseDynamicMeshComponent.GetDynamicMesh` (`self.DynamicMeshComponent`)))
    (bind _returnvalue_4 (`GeometryScriptLibrary_MeshTransformFunctions.TranslateMesh` _returnvalue_3 (`KismetMathLibrary.MakeVector` 0.0 0.0 _roof_location_z) null))
    (if (`self.Flip Normal`)
      (`GeometryScriptLibrary_MeshNormalsFunctions.FlipNormals` _returnvalue_4 null))))

(fn `UserConstructionScript`
  (if (`self.Activate Spline Edition`)
    (`/Game/ProceduralBuildingGenerator/Blueprints/Library/PBG_Functions.PBG Auto Correct Spline Orientation` (`self.Spline`))
    (bind _points (`/Game/ProceduralBuildingGenerator/Blueprints/Library/PBG_Functions.PBG Get Spline Points` (`self.Spline`) "Local"))
    (set `self.Vertex` _points)))