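; Homing projectile weapon that sweeps forward each tick and deals radial falloff damage on capsule overlap, sparing PlayerRef.
; After a delay it steers by rotation lerp toward CurrentTarget, leading moving distant targets, with aim computed from PlayerRef's transform rather than its own.
; Fuel sets lifespan and gates acceleration versus slowdown with weaker turning, but its per-tick decrement is zero.
; Movement feeds the world forward vector into a local offset.
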(event `self.ReceiveBeginPlay`
  (`self.SetLifeSpan` (+ (`self.Fuel`) 10.0)))

(event `self.ReceiveTick`
  (params (DeltaSeconds :type "Float (single-precision)"))
  (bind _returnvalue (`GameplayStatics.GetWorldDeltaSeconds`))
  (if (`self.IsHoming`)
    (if (> (`self.Fuel`) 0.0)
      (set `self.CurrentSpeedM` (`KismetMathLibrary.FInterpTo` (`self.CurrentSpeedM`) (`self.ThrustSpeedM`) 0.0 0.1))
      (set `self.Fuel` (- (`self.Fuel`) 0.0))
      (`self.FollowTarget` (`self.Turnspeed`))
      (else
        (set `self.CurrentSpeedM` (- (`self.CurrentSpeedM`) (* DeltaSeconds 5.0)))
        (`self.FollowTarget` (* (`self.Turnspeed`) 0.2)))))
  (`self.K2_AddActorLocalOffset` (* (`self.GetActorForwardVector`) (`self.CurrentSpeedM`) (`self.SpeedMultiplier`) _returnvalue) true)
  (if (== (`self.HomingDelay`) 0.0)
    (`/Engine/EditorBlueprintResources/StandardMacros.DoOnce` false
      (:`Completed`
        (set `self.IsHoming` true)
        (set `self.IsDeployed` true)))
    (else
      (set `self.HomingDelay` (`KismetMathLibrary.FClamp` (- (`self.HomingDelay`) _returnvalue) 0.0 10.0)))))

(event `self.Capsule.OnComponentBeginOverlap`
  (params (OverlappedComponent :type "PrimitiveComponent Object Reference") (OtherActor :type "Actor Object Reference") (OtherComp :type "PrimitiveComponent Object Reference") (OtherBodyIndex :type Integer) (bFromSweep :type Boolean) (SweepResult :type "HitResult Structure (by ref)"))
  (`GameplayStatics.ApplyRadialDamageWithFalloff` (`self.Damage`) 35.0 (`.ImpactPoint` (`GameplayStatics.BreakHitResult` SweepResult)) 10.0 39.0 0.0 "/Script/Engine.DamageType" (`|MakeArray` (`self.PlayerRef`) :!type "Actor Object Reference") self null))

(fn `FollowTarget`
  (params (Turnspeed :type "Float (double-precision)"))
  (bind _currenttarget (`self.CurrentTarget`))
  (bind _returnvalue (`self.K2_GetActorLocation` _currenttarget))
  (bind (_returnvalue_location _returnvalue_rotation) (`KismetMathLibrary.BreakTransform` (`self.GetTransform` (`self.PlayerRef`))))
  (bind _returnvalue_2 (`KismetMathLibrary.Vector_Distance` _returnvalue _returnvalue_location))
  (bind _returnvalue_3 (`KismetMathLibrary.VSize` (`self.GetVelocity` _currenttarget)))
  (`/Engine/EditorBlueprintResources/StandardMacros.IsValid` _currenttarget
    (:`Is Valid`
      (`self.K2_SetActorRotation` (`KismetMathLibrary.RLerp` _returnvalue_rotation (`KismetMathLibrary.FindLookAtRotation` _returnvalue_location (select `bool` (or (< _returnvalue_2 100.0) (< _returnvalue_3 10.0)) :`false` (+ _returnvalue (* (`self.GetActorForwardVector` _currenttarget) (* (* _returnvalue_3 0.001) (* _returnvalue_2 0.001)))) :`true` _returnvalue)) (* Turnspeed 0.1) true)))))

(fn `UserConstructionScript`
  (`parent.UserConstructionScript`))