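; Test actor for the Procedural City Creator that builds two spline-swept dynamic meshes and measures how close they are.
; The construction script resamples each spline by length and sweeps a shared 2D profile along it with Geometry Script, recomputing normals.
; It then runs intersection and distance queries between the meshes and prints the minimum distance.
; The branch on the intersection result is disconnected, and the event graph is empty.
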(fn `Create Mesh`
  (locals (TA :type "Array of Transform Structure") (`2DVertices` :type "Array of Vector2D Structure"))
  (bind _vertices (`/Game/ProceduralCityCreator/Library/PCC_Functions.PCC Set Path Vertices` -100.0 500.0))
  (set `local.2DVertices` _vertices)
  (bind (_valid _spoints _transforms) (`/Game/ProceduralCityCreator/Library/PCC_Functions.PCC Resample Spline By Length` (`self.Spline`) 500.0 "Local" true))
  (set `local.TA` _transforms)
  (bind _returnvalue (`BaseDynamicMeshComponent.GetDynamicMesh` (`self.DynamicMesh`)))
  (bind _returnvalue_2 (`DynamicMesh.Reset` _returnvalue))
  (bind _output_get (set `self.Dyna A` _returnvalue_2))
  (bind _returnvalue_3 (`GeometryScriptLibrary_MeshPrimitiveFunctions.AppendSweepPolygon` _output_get (struct) (struct) (`local.2DVertices`) (`local.TA`) false true 1.0 1.0 0.0 null))
  (bind _returnvalue_4 (`GeometryScriptLibrary_MeshNormalsFunctions.RecomputeNormals` _returnvalue_3 (struct) null))
  (`GeometryScriptLibrary_MeshNormalsFunctions.ComputeSplitNormals` _returnvalue_4 (struct) (struct) null)
  (bind (_valid_2 _spoints_2 _transforms_2) (`/Game/ProceduralCityCreator/Library/PCC_Functions.PCC Resample Spline By Length` (`self.Spline_B`) 500.0 "Local" true))
  (set `local.TA` _transforms_2)
  (bind _returnvalue_5 (`BaseDynamicMeshComponent.GetDynamicMesh` (`self.DynamicMeshB`)))
  (bind _returnvalue_6 (`DynamicMesh.Reset` _returnvalue_5))
  (bind _output_get_2 (set `self.Dyna B` _returnvalue_6))
  (bind _returnvalue_7 (`GeometryScriptLibrary_MeshPrimitiveFunctions.AppendSweepPolygon` _output_get_2 (struct) (struct) (`local.2DVertices`) (`local.TA`) false true 1.0 1.0 0.0 null))
  (bind _returnvalue_8 (`GeometryScriptLibrary_MeshNormalsFunctions.RecomputeNormals` _returnvalue_7 (struct) null))
  (`GeometryScriptLibrary_MeshNormalsFunctions.ComputeSplitNormals` _returnvalue_8 (struct) (struct) null)
  (bind _bisintersecting (`GeometryScriptLibrary_MeshComparisonFunctions.IsIntersectingMesh` (`self.Dyna A`) (struct) (`self.Dyna B`) (struct) null))
  (bind (_maxdistance _mindistance) (`GeometryScriptLibrary_MeshComparisonFunctions.MeasureDistancesBetweenMeshes` (`self.Dyna A`) (`self.Dyna B`) (struct) null))
  (`KismetSystemLibrary.PrintString` (`KismetStringLibrary.Conv_DoubleToString` _mindistance) true true (struct :`G` 0.66 :`B` 1.0 :`A` 1.0) 0.3))

(fn `UserConstructionScript`
  (`self.Create Mesh`))