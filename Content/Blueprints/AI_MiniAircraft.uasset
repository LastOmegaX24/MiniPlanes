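; AI-controlled mini aircraft that attacks pawns it senses and can be shot down or crash.
; Close targets get gated gun bursts with ammo and reload, multicast through RPCs; farther targets get a delayed missile.
; RPCExplode switches off AIMiniMove, enables physics, optionally adds fire and removes "rdr"-tagged attachments.
; Collisions trigger an explosion and delayed destruction, usually with lethal self-damage unless already crashing.
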(event `self.ReceiveTick`
  (params (DeltaSeconds :type "Float (single-precision)"))
  (if (not (`self.Crashing`))
    (`parent.ReceiveTick` DeltaSeconds)))

(event `self.ReceiveBeginPlay`
  (`parent.ReceiveBeginPlay`))

(event `self.ReceiveRestarted`)

(event `self.ReceiveAnyDamage`
  (params (Damage :type "Float (single-precision)") (DamageType :type "DamageType Object Reference") (InstigatedBy :type "Controller Object Reference") (DamageCauser :type "Actor Object Reference"))
  (`parent.ReceiveAnyDamage` Damage DamageType InstigatedBy DamageCauser))

(event `self.RPC_Explode`
  (params (Burning :type Boolean))
  (set `self.Crashing` true)
  (`GMC_ReplicationCmp.EnableGMC` (`self.AI_MiniMove`) false)
  (`PrimitiveComponent.SetSimulatePhysics` (`self.Box1`) true)
  (`SceneComponent.SetVisibility` (`self.HealthBar`) false false)
  (if Burning
    (`GameplayStatics.SpawnEmitterAttached` "/Engine/Tutorial/SubEditors/TutorialAssets/TutorialParticleSystem.TutorialParticleSystem" null "None" (0.0 0.0 0.0) (struct) (2.0 2.0 2.0)))
  (for _array_element (`self.GetAttachedActors` true)
    (if (`self.ActorHasTag` _array_element "rdr")
      (`self.K2_DestroyActor` _array_element))))

(event `self.PawnSensing.OnSeePawn`
  (params (Pawn :type "Pawn Object Reference"))
  (set `self.LockTarget` Pawn)
  (if (< (`self.GetDistanceTo` Pawn self) 500.0)
    (`|ExecutionSequence`
      (:`then_0`
        (`|ExecutionSequence`
          (:`then_0`
            (goto _label :!via `Open`))
          (:`then_1`
            (if (`self.CanShoot`)
              (`/Engine/EditorBlueprintResources/StandardMacros.Gate` true :!label _label
                (:`Exit`
                  (set `self.CanShoot` false)
                  (if (and (> (`self.Ammo`) 0) (not (`/Game/Blueprints/AI_MiniMove.IsCobra` (`self.AI_MiniMove`))))
                    (`/Engine/EditorBlueprintResources/StandardMacros.DecrementInt` (`self.Ammo`)
                      (:`  `
                        (`self.RPC_ShootGun` null)))
                    (else
                      (`self.Reload`)))
                  (`KismetSystemLibrary.Delay` (`.FireInterval_71_166CC40548844735102D93B0C6909171` (break `/Game/AircraftData/AircraftDataStructure` (`self.AircraftData`))))
                  (set `self.CanShoot` true)
                  (goto _label)))))))
      (:`then_1`
        (`KismetSystemLibrary.Delay` 0.4)
        (goto _label :!via `Close`)))
    (else
      (`KismetSystemLibrary.Delay` 5.0)
      (`self.ShootMissile` (`/Game/Blueprints/AI_MiniMove.CurrentSpeed` (`self.AI_MiniMove`))))))

(event `Reload`
  (bind (_maxthrust _maxspeed _minspeedstall _acceleration _brakespeed _turnspeed _ratespeed _maxhealth _maxammo _reservemissiles _reloadtime) (break `/Game/AircraftData/AircraftDataStructure` (`self.AircraftData`)))
  (set `self.Ammo` 0)
  (`KismetSystemLibrary.Delay` _reloadtime)
  (set `self.Ammo` _maxammo))

(event `RPC_Multi_ShootGun`
  (params (ParentPlayer :type "/Game/Blueprints/Aircraft Object Reference"))
  (`self.OVR_ShootAll` ParentPlayer))

(event `OVR_ShootAll`
  (params (ParentPlayer :type "/Game/Blueprints/Aircraft Object Reference"))
  (bind (_maxthrust _maxspeed _minspeedstall _acceleration _brakespeed _turnspeed _ratespeed _maxhealth _maxammo _reservemissiles _reloadtime _rcs _gunaccuracy _gundamage) (break `/Game/AircraftData/AircraftDataStructure` (`self.AircraftData`)))
  (if (not (`self.Crashing`))
    (`self.ShootGunF` true _gunaccuracy _gundamage ParentPlayer (`/Game/Blueprints/AI_MiniMove.CurrentSpeed` (`self.AI_MiniMove`)))))

(event `RPC_ShootGun`
  (params (ParentPlayer :type "/Game/Blueprints/BP_MiniAircraft Object Reference"))
  (`self.RPC_Multi_ShootGun` ParentPlayer))

(event `SelfDamage`
  (params (BaseDamage :type "Float (single-precision)"))
  (`GameplayStatics.ApplyDamage` self BaseDamage null self "/Engine/EngineDamageTypes/DmgTypeBP_Environmental.DmgTypeBP_Environmental_C"))

(event `self.ReceiveHit`
  (params (MyComp :type "PrimitiveComponent Object Reference") (Other :type "Actor Object Reference") (OtherComp :type "PrimitiveComponent Object Reference") (bSelfMoved :type Boolean) (HitLocation :type "Vector Structure") (HitNormal :type "Vector Structure") (NormalImpulse :type "Vector Structure") (Hit :type "HitResult Structure (by ref)"))
  (if (not (== Other self))
    (if (`self.ActorHasTag` Other "Entity")
      (if (`self.Crashing`)
        (`/Engine/EditorBlueprintResources/StandardMacros.DoOnce` false
          (:`Completed`
            (`self.RPC_Server_Destroy` HitLocation :!label _label_2)))
        (else
          (`/Engine/EditorBlueprintResources/StandardMacros.DoOnce` false
            (:`Completed`
              (`self.SelfDamage` 999999.0)
              (`self.RPC_Server_Destroy` HitLocation)))))
      (else
        (`/Engine/EditorBlueprintResources/StandardMacros.DoOnce` false
          (:`Completed`
            (`self.SelfDamage` 999999.0)
            (goto _label_2)))))))

(event `RPC_Server_Destroy`
  (params (Location :type "Vector Structure"))
  (`self.RPC_CrashParticle` Location)
  (`KismetSystemLibrary.Delay` 10.0)
  (`self.K2_DestroyActor`))

(event `RPC_CrashParticle`
  (params (Location :type "Vector Structure"))
  (`GameplayStatics.SpawnEmitterAtLocation` "/Game/Realistic_Starter_VFX_Pack_Vol2/Particles/Explosion/P_Explosion_Big_A.P_Explosion_Big_A" Location))

(fn `ResetVar`)

(fn `UserConstructionScript`
  (`parent.UserConstructionScript`))