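; Optimized mesh actor from the Procedural Building Generator that holds one mesh as ISM or HISM instances, with utility functions to manage them.
; Conversion functions copy mesh, materials and transforms between the two components, then clear and hide the source.
; Release functions spawn a tagged StaticMeshActor per instance without clearing the instances.
; Other functions toggle physics with mobility, shadows and cull distances, most updating status strings.
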(fn `Activate Physics`
  (`StaticMeshComponent.StaticMesh` (`self.HierarchicalInstancedStaticMesh`)
    (:`then`
      (`SceneComponent.SetMobility` (`self.HierarchicalInstancedStaticMesh`) "Movable")
      (`PrimitiveComponent.SetSimulatePhysics` (`self.HierarchicalInstancedStaticMesh`) true))
    (:`else`
      (`StaticMeshComponent.StaticMesh` (`self.InstancedStaticMesh`)
        (:`then`
          (`SceneComponent.SetMobility` (`self.InstancedStaticMesh`) "Movable")
          (`PrimitiveComponent.SetSimulatePhysics` (`self.InstancedStaticMesh`) true))
        (:`else`))))
  (set `self.Physic State` "Has Mobility and Physics enabled"))

(fn `Convert HISM to ISM`
  (locals (`Mesh Actor Ref` :type "StaticMeshActor Object Reference") (Valid :type Boolean :default false) (`Error Count` :type Integer))
  (bind _hierarchicalinstancedstaticmesh (`self.HierarchicalInstancedStaticMesh`))
  (`StaticMeshComponent.StaticMesh` (`self.HierarchicalInstancedStaticMesh`)
    (:`then`
      (`StaticMeshComponent.SetStaticMesh` (`self.InstancedStaticMesh`) (`StaticMeshComponent.StaticMesh` (`self.HierarchicalInstancedStaticMesh`)))
      (for (_array_element _array_index) (`MeshComponent.GetMaterials` (`self.HierarchicalInstancedStaticMesh`))
        (`PrimitiveComponent.SetMaterial` (`self.InstancedStaticMesh`) _array_index _array_element))
      (for _index (range (`InstancedStaticMeshComponent.GetInstanceCount` _hierarchicalinstancedstaticmesh))
        (bind (_outinstancetransform _returnvalue) (`InstancedStaticMeshComponent.GetInstanceTransform` _hierarchicalinstancedstaticmesh _index true))
        (if _returnvalue
          (set `local.Valid` true)
          (`InstancedStaticMeshComponent.AddInstance` (`self.InstancedStaticMesh`) _outinstancetransform true)
          (else
            (`KismetSystemLibrary.PrintString` (`KismetStringLibrary.Concat_StrStr` "instance: " (`KismetStringLibrary.Conv_IntToString` _index) " \ncan't be released") true true (struct :`R` 1.0 :`A` 1.0) 5.0)
            (`/Engine/EditorBlueprintResources/StandardMacros.IncrementInt` (`local.Error Count`)))))
      (if (`local.Valid`)
        (set `self.Current Instance Type` "ISM (instanced static mesh)")
        (`KismetSystemLibrary.PrintString` (`KismetStringLibrary.Concat_StrStr` "HISM to ISM Convertion \ncompleted." (select `bool` (!= (`local.Error Count`) 0) :`false` "!" :`true` (`KismetStringLibrary.Concat_StrStr` " with: " (`KismetStringLibrary.Conv_IntToString` (`local.Error Count`)) " errors"))) true true (struct :`G` 1.0 :`A` 1.0) 5.0)
        (`InstancedStaticMeshComponent.ClearInstances` (`self.HierarchicalInstancedStaticMesh`))
        (`StaticMeshComponent.SetStaticMesh` (`self.HierarchicalInstancedStaticMesh`) null)
        (`SceneComponent.SetVisibility` (`self.HierarchicalInstancedStaticMesh`) false false)
        (`SceneComponent.SetVisibility` (`self.InstancedStaticMesh`) true false)
        (else
          (`KismetSystemLibrary.PrintString` "No Instances were released" true true (struct :`R` 1.0 :`A` 1.0) 5.0))))
    (:`else`
      (`KismetSystemLibrary.PrintString` "cannot convert, no mesh found"))))

(fn `Convert ISM to HISM`
  (locals (`Mesh Actor Ref` :type "StaticMeshActor Object Reference") (Valid :type Boolean :default false) (`Error Count` :type Integer))
  (bind _instancedstaticmesh (`self.InstancedStaticMesh`))
  (`StaticMeshComponent.StaticMesh` (`self.InstancedStaticMesh`)
    (:`then`
      (`StaticMeshComponent.SetStaticMesh` (`self.HierarchicalInstancedStaticMesh`) (`StaticMeshComponent.StaticMesh` (`self.InstancedStaticMesh`)))
      (for (_array_element _array_index) (`MeshComponent.GetMaterials` (`self.InstancedStaticMesh`))
        (`PrimitiveComponent.SetMaterial` (`self.HierarchicalInstancedStaticMesh`) _array_index _array_element))
      (for _index (range (`InstancedStaticMeshComponent.GetInstanceCount` _instancedstaticmesh))
        (bind (_outinstancetransform _returnvalue) (`InstancedStaticMeshComponent.GetInstanceTransform` _instancedstaticmesh _index true))
        (if _returnvalue
          (set `local.Valid` true)
          (`InstancedStaticMeshComponent.AddInstance` (`self.HierarchicalInstancedStaticMesh`) _outinstancetransform true)
          (else
            (`KismetSystemLibrary.PrintString` (`KismetStringLibrary.Concat_StrStr` "instance: " (`KismetStringLibrary.Conv_IntToString` _index) " \ncan't be released") true true (struct :`R` 1.0 :`A` 1.0) 5.0)
            (`/Engine/EditorBlueprintResources/StandardMacros.IncrementInt` (`local.Error Count`)))))
      (if (`local.Valid`)
        (set `self.Current Instance Type` "HISM (hierarchical instanced static mesh)")
        (`KismetSystemLibrary.PrintString` (`KismetStringLibrary.Concat_StrStr` "ISM to HISM Convertion \ncompleted." (select `bool` (!= (`local.Error Count`) 0) :`false` "!" :`true` (`KismetStringLibrary.Concat_StrStr` " with: " (`KismetStringLibrary.Conv_IntToString` (`local.Error Count`)) " errors"))) true true (struct :`G` 1.0 :`A` 1.0) 5.0)
        (`InstancedStaticMeshComponent.ClearInstances` (`self.InstancedStaticMesh`))
        (`StaticMeshComponent.SetStaticMesh` (`self.InstancedStaticMesh`) null)
        (`SceneComponent.SetVisibility` (`self.InstancedStaticMesh`) false false)
        (`SceneComponent.SetVisibility` (`self.HierarchicalInstancedStaticMesh`) true false)
        (else
          (`KismetSystemLibrary.PrintString` "No Instances were released" true true (struct :`R` 1.0 :`A` 1.0) 5.0))))
    (:`else`
      (`KismetSystemLibrary.PrintString` "cannot convert, no mesh found"))))

(fn `Disable Shadow`
  (`PrimitiveComponent.SetCastShadow` (`self.InstancedStaticMesh`) false)
  (`PrimitiveComponent.SetCastShadow` (`self.HierarchicalInstancedStaticMesh`) false)
  (set `self.Shadow State` "No shadow enabled"))

(fn `Enable Shadow`
  (`PrimitiveComponent.SetCastShadow` (`self.InstancedStaticMesh`) true)
  (`PrimitiveComponent.SetCastShadow` (`self.HierarchicalInstancedStaticMesh`) true)
  (set `self.Shadow State` "Shadow is actived."))

(fn `Release All HISM Instances`
  (locals (`Mesh Actor Ref` :type "StaticMeshActor Object Reference") (Valid :type Boolean :default false) (`Error Count` :type Integer))
  (bind _hierarchicalinstancedstaticmesh (`self.HierarchicalInstancedStaticMesh`))
  (`StaticMeshComponent.StaticMesh` (`self.HierarchicalInstancedStaticMesh`)
    (:`then`
      (for _index (range (`InstancedStaticMeshComponent.GetInstanceCount` _hierarchicalinstancedstaticmesh))
        (bind (_outinstancetransform _returnvalue) (`InstancedStaticMeshComponent.GetInstanceTransform` _hierarchicalinstancedstaticmesh _index true))
        (if _returnvalue
          (set `local.Valid` true)
          (bind _returnvalue_2 (`|SpawnActorFromClass` "/Script/Engine.StaticMeshActor" _outinstancetransform "AlwaysSpawn" "MultiplyWithRoot" null null))
          (bind _output_get (set `local.Mesh Actor Ref` _returnvalue_2))
          (`StaticMeshComponent.SetStaticMesh` (`StaticMeshActor.StaticMeshComponent` _output_get) (`StaticMeshComponent.StaticMesh` (`self.HierarchicalInstancedStaticMesh`)))
          (bind _output_get_2 (set `Actor.Tags` (`self.Tags`) (`local.Mesh Actor Ref`)))
          (`KismetArrayLibrary.Array_AddUnique` _output_get_2 (`self.OptiZ Tag`))
          (for (_array_element _array_index) (`MeshComponent.GetMaterials` (`self.HierarchicalInstancedStaticMesh`))
            (`PrimitiveComponent.SetMaterial` (`StaticMeshActor.StaticMeshComponent` (`local.Mesh Actor Ref`)) _array_index _array_element))
          (else
            (`KismetSystemLibrary.PrintString` (`KismetStringLibrary.Concat_StrStr` "instance: " (`KismetStringLibrary.Conv_IntToString` _index) " \ncan't be released") true true (struct :`R` 1.0 :`A` 1.0) 5.0)
            (`/Engine/EditorBlueprintResources/StandardMacros.IncrementInt` (`local.Error Count`))))))
    (:`else`
      _))
  (if (`local.Valid`)
    (`KismetSystemLibrary.PrintString` (`KismetStringLibrary.Concat_StrStr` "Release Completed" (select `bool` (!= (`local.Error Count`) 0) :`false` "!" :`true` (`KismetStringLibrary.Concat_StrStr` " with: " (`KismetStringLibrary.Conv_IntToString` (`local.Error Count`)) " errors"))) true true (struct :`G` 1.0 :`A` 1.0) 5.0)
    (else
      (`KismetSystemLibrary.PrintString` "No Instances were released" true true (struct :`R` 1.0 :`A` 1.0) 5.0))))

(fn `Release All ISM Instances`
  (locals (`Mesh Actor Ref` :type "StaticMeshActor Object Reference") (Valid :type Boolean :default false) (`Error Count` :type Integer))
  (bind _instancedstaticmesh (`self.InstancedStaticMesh`))
  (`StaticMeshComponent.StaticMesh` (`self.InstancedStaticMesh`)
    (:`then`
      (for _index (range (`InstancedStaticMeshComponent.GetInstanceCount` _instancedstaticmesh))
        (bind (_outinstancetransform _returnvalue) (`InstancedStaticMeshComponent.GetInstanceTransform` _instancedstaticmesh _index true))
        (if _returnvalue
          (set `local.Valid` true)
          (bind _returnvalue_2 (`|SpawnActorFromClass` "/Script/Engine.StaticMeshActor" _outinstancetransform "AlwaysSpawn" "MultiplyWithRoot" null null))
          (bind _output_get (set `local.Mesh Actor Ref` _returnvalue_2))
          (`StaticMeshComponent.SetStaticMesh` (`StaticMeshActor.StaticMeshComponent` _output_get) (`StaticMeshComponent.StaticMesh` (`self.InstancedStaticMesh`)))
          (bind _output_get_2 (set `Actor.Tags` (`self.Tags`) (`local.Mesh Actor Ref`)))
          (`KismetArrayLibrary.Array_AddUnique` _output_get_2 (`self.OptiZ Tag`))
          (for (_array_element _array_index) (`MeshComponent.GetMaterials` (`self.InstancedStaticMesh`))
            (`PrimitiveComponent.SetMaterial` (`StaticMeshActor.StaticMeshComponent` (`local.Mesh Actor Ref`)) _array_index _array_element))
          (else
            (`KismetSystemLibrary.PrintString` (`KismetStringLibrary.Concat_StrStr` "instance: " (`KismetStringLibrary.Conv_IntToString` _index) " \ncan't be released") true true (struct :`R` 1.0 :`A` 1.0) 5.0)
            (`/Engine/EditorBlueprintResources/StandardMacros.IncrementInt` (`local.Error Count`))))))
    (:`else`
      _))
  (if (`local.Valid`)
    (`KismetSystemLibrary.PrintString` (`KismetStringLibrary.Concat_StrStr` "Release Completed" (select `bool` (!= (`local.Error Count`) 0) :`false` "!" :`true` (`KismetStringLibrary.Concat_StrStr` " with: " (`KismetStringLibrary.Conv_IntToString` (`local.Error Count`)) " errors"))) true true (struct :`G` 1.0 :`A` 1.0) 5.0)
    (else
      (`KismetSystemLibrary.PrintString` "No Instances were released" true true (struct :`R` 1.0 :`A` 1.0) 5.0))))

(fn `Remove Physics`
  (`StaticMeshComponent.StaticMesh` (`self.HierarchicalInstancedStaticMesh`)
    (:`then`
      (`SceneComponent.SetMobility` (`self.HierarchicalInstancedStaticMesh`) "Static")
      (`PrimitiveComponent.SetSimulatePhysics` (`self.HierarchicalInstancedStaticMesh`) false))
    (:`else`
      (`StaticMeshComponent.StaticMesh` (`self.InstancedStaticMesh`)
        (:`then`
          (`SceneComponent.SetMobility` (`self.InstancedStaticMesh`) "Static")
          (`PrimitiveComponent.SetSimulatePhysics` (`self.InstancedStaticMesh`) false))
        (:`else`))))
  (set `self.Physic State` "No Physics"))

(fn `Set Culling Distance`
  (`InstancedStaticMeshComponent.SetCullDistances` (`self.HierarchicalInstancedStaticMesh`) (`self.Start Cull Distance`) (`self.End Cull Distance`))
  (`InstancedStaticMeshComponent.SetCullDistances` (`self.InstancedStaticMesh`) (`self.Start Cull Distance`) (`self.End Cull Distance`)))

(fn `UserConstructionScript`)