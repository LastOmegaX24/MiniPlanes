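; AOE_Wep is an expanding area-of-effect blast actor that damages each overlapping actor once, excluding its Parent.
; After a blast delay at start radius, Tick interpolates Sphere1's scale toward the explosion radius, then destroys the actor following a hold time.
; A dynamic material on Plane receives the radius ratio as its "time" parameter, keeping the visual in step with the expansion.
; Overlaps apply PlayerDamage attributed to Parent, using the AlreadyHit array to block repeat hits.
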(event `self.ReceiveBeginPlay`
  (bind _plane (`self.Plane`))
  (bind _returnvalue (`PrimitiveComponent.CreateDynamicMaterialInstance` _plane 0 (`PrimitiveComponent.GetMaterial` _plane 0) "None"))
  (bind _output_get (set `self.MaterialInst` _returnvalue))
  (`PrimitiveComponent.SetMaterial` (`self.Plane`) 0 _output_get))

(event `self.ReceiveTick`
  (params (DeltaSeconds :type "Float (single-precision)"))
  (bind _materialinst (`self.MaterialInst`))
  (bind _startradius (`self.StartRadius`))
  (`/Engine/EditorBlueprintResources/StandardMacros.IsValid` _materialinst
    (:`Is Valid`
      (`MaterialInstanceDynamic.SetScalarParameterValue` _materialinst "time" (`KismetMathLibrary.SafeDivide` (`self.CurrentRadius`) (`self.ExplosionRadius`)))
      (if (> (`self.CurrentDelay`) (`self.BlastDelay`))
        (bind _output_get (set `self.CurrentRadius` (`KismetMathLibrary.FInterpTo` (`self.CurrentRadius`) (`self.ExplosionRadius`) DeltaSeconds (`self.ExpansionSpeed`))))
        (`SceneComponent.SetRelativeScale3D` (`self.Sphere1`) (`KismetMathLibrary.MakeVector` _output_get _output_get _output_get))
        (if (>= (+ (`self.CurrentRadius`) 0.1) (`self.ExplosionRadius`))
          (`/Engine/EditorBlueprintResources/StandardMacros.DoOnce` false
            (:`Completed`
              (`KismetSystemLibrary.Delay` (`self.HoldTime`))
              (`self.K2_DestroyActor`))))
        (else
          (set `self.CurrentDelay` (+ (`self.CurrentDelay`) DeltaSeconds))
          (`SceneComponent.SetRelativeScale3D` (`self.Sphere1`) (`KismetMathLibrary.MakeVector` _startradius _startradius _startradius)))))))

(event `self.ReceiveActorBeginOverlap`
  (params (OtherActor :type "Actor Object Reference"))
  (bind _parent (`self.Parent`))
  (if (and (!= _parent OtherActor) (== (`KismetArrayLibrary.Array_Find` (`self.AlreadyHit`) OtherActor) -1))
    (`GameplayStatics.ApplyDamage` OtherActor (`self.Damage`) null _parent "/Game/Blueprints/DamageType/PlayerDamage.PlayerDamage_C")
    (`KismetArrayLibrary.Array_Add` (`self.AlreadyHit`) OtherActor)))

(fn `UserConstructionScript`
  (set `self.CurrentRadius` (`self.StartRadius`)))