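; F22 plane Blueprint that tints its mesh with a configurable color when play begins.
; After the parent BeginPlay, it creates a dynamic instance of PlaneMesh's first material, sets its Color parameter from PlaneColor and applies it to the mesh.
; The construction script only calls the parent, and the overlap and Tick events are disabled stubs.
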(event `self.ReceiveBeginPlay`
  (bind _planemesh (`self.PlaneMesh`))
  (`parent.ReceiveBeginPlay`)
  (bind _returnvalue (`PrimitiveComponent.CreateDynamicMaterialInstance` _planemesh 0 (`PrimitiveComponent.GetMaterial` _planemesh 0) "None"))
  (`MaterialInstanceDynamic.SetVectorParameterValue` _returnvalue "Color" (`self.PlaneColor`))
  (`PrimitiveComponent.SetMaterial` _planemesh 0 _returnvalue))

(fn `UserConstructionScript`
  (`parent.UserConstructionScript`))