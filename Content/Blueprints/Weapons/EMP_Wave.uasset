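; EMP wave weapon actor that applies a timed effect to aircraft and homing weapons it touches.
; On overlap it calls the parent handler, ignores invalid actors and its Parent, then casts the other actor to Aircraft or HomingWep.
; A match receives a component of the configured Class with a fixed duration and no delay, so the effect logic lives in that component.
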(event `self.ReceiveActorBeginOverlap`
  (params (OtherActor :type "Actor Object Reference"))
  (bind _class (`self.Class`))
  (`parent.ReceiveActorBeginOverlap` OtherActor)
  (`/Engine/EditorBlueprintResources/StandardMacros.IsValid` OtherActor
    (:`Is Valid`
      (if (!= OtherActor (`self.Parent`))
        (bind _asaircraft (cast `/Game/Blueprints/Aircraft` OtherActor)
          (:`then`
            (`|AddComponentByClass` _asaircraft _class 10.0 0.0))
          (:`CastFailed`
            (bind _ashoming_wep (cast `/Game/Blueprints/Weapons/HomingWep` OtherActor))
            (`|AddComponentByClass` _ashoming_wep _class 10.0 0.0)))))))

(fn `UserConstructionScript`
  (`parent.UserConstructionScript`))