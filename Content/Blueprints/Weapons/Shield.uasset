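; Timed shield actor that absorbs damage into a health pool, scaled by Radius and expiring after Duration.
; Damage tallies BlockedDamage and drains Health; at zero it breaks and is either destroyed or deactivated.
; Optional regeneration calls Activate at a threshold and drives material opacity below it, though Activate, like Deactivate, hides the mesh and disables collision.
; A widget health bar references the shield, and EndPlay notifies the parent that the ability ended.
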(event `self.ReceiveBeginPlay`
  (bind _staticmesh (`self.StaticMesh`))
  (bind _returnvalue (`PrimitiveComponent.CreateDynamicMaterialInstance` _staticmesh 0 (`PrimitiveComponent.GetMaterial` _staticmesh 0) "None"))
  (set `self.DynamicShieldmat` _returnvalue)
  (bind _asshield_health_bar (cast `/Game/UI/ShieldHealthBar` (`WidgetComponent.GetWidget` (`self.Widget`))))
  (set `/Game/UI/ShieldHealthBar.OwnerRef` self _asshield_health_bar))

(event `self.ReceiveAnyDamage`
  (params (Damage :type "Float (single-precision)") (DamageType :type "DamageType Object Reference") (InstigatedBy :type "Controller Object Reference") (DamageCauser :type "Actor Object Reference"))
  (set `self.BlockedDamage` (+ (`self.BlockedDamage`) Damage))
  (bind _output_get (set `self.Health` (- (`self.Health`) Damage)))
  (if (<= _output_get 0.0)
    (set `self.Broken` true)
    (if (`self.DestroyIfDisabled`)
      (`self.K2_DestroyActor`)
      (else
        (`self.Deactivate`)))))

(event `self.ReceiveTick`
  (params (DeltaSeconds :type "Float (single-precision)"))
  (if (`self.Regenerate`)
    (bind _output_get (set `self.Health` (`KismetMathLibrary.FClamp` (+ (* DeltaSeconds (`self.RegenRate`)) (`self.Health`)) 0.0 (`self.MaxHealth`))))
    (if (>= _output_get (`self.ActivationThreshhold`))
      (`/Engine/EditorBlueprintResources/StandardMacros.DoOnce` false :!label _label
        (:`Completed`
          (`self.Activate`)))
      (else
        (`|ExecutionSequence`
          (:`then_0`
            (goto _label :!via `Reset`))
          (:`then_1`
            (`MaterialInstanceDynamic.SetScalarParameterValue` (`self.DynamicShieldmat`) "Opacity" (`KismetMathLibrary.SafeDivide` _output_get (`self.MaxHealth`)))))))))

(event `Activate`
  (bind _staticmesh (`self.StaticMesh`))
  (set `self.Broken` false)
  (`SceneComponent.SetVisibility` _staticmesh false false)
  (`PrimitiveComponent.SetCollisionEnabled` _staticmesh "NoCollision"))

(event `Deactivate`
  (bind _staticmesh (`self.StaticMesh`))
  (`SceneComponent.SetVisibility` _staticmesh false false)
  (`PrimitiveComponent.SetCollisionEnabled` _staticmesh "NoCollision"))

(event `self.ReceiveEndPlay`
  (params (EndPlayReason :type "EEndPlayReason Enum" :default "Destroyed"))
  (message `/Game/Blueprints/Interface/AbilityStatus.AbilityEnded` (`self.Parent`)))

(fn `UserConstructionScript`
  (bind _radius (`self.Radius`))
  (`SceneComponent.SetWorldScale3D` (`self.StaticMesh`) (`KismetMathLibrary.MakeVector` _radius _radius _radius))
  (`self.SetLifeSpan` (`self.Duration`)))