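; PROTOTYPE_9 is a plane Blueprint whose special ability spawns a PTT_Shield attached to its Arrow0 component.
; Tick drives thruster effects on four meshes from the afterburner state and recharges the ability over the aircraft's cooldown while it is inactive.
; Ability input spends the charge and routes activation through parent RPCs by authority, with the OVRAbility override supplying the shield spawn.
; InAbility pauses recharge and is not cleared in this graph.
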(event `self.ReceiveTick`
  (params (DeltaSeconds :type "Float (single-precision)"))
  (`parent.ReceiveTick` DeltaSeconds)
  (`self.CreateThruster` (`|MakeArray` (`self.StaticMesh3`) (`self.StaticMesh2`) (`self.StaticMesh4`) (`self.StaticMesh1`) :!type "PrimitiveComponent Object Reference") (`/Game/Blueprints/MiniMove.IsAfterburner` (`self.MiniMove`)))
  (if (not (`self.InAbility`))
    (bind _output_get (set `self.AbilityCharge` (`KismetMathLibrary.FClamp` (+ (`self.AbilityCharge`) (`KismetMathLibrary.SafeDivide` DeltaSeconds (`.AbilityCooldown_79_D58A382A446A2EC56EA71AB0D5CB7B1F` (break `/Game/AircraftData/AircraftDataStructure` (`self.AircraftData`))))))))
    (if (== _output_get 1.0)
      (set `self.IsAbilityReady` true))))

(event `self.OVR_Ability`
  (bind _returnvalue_location (`KismetMathLibrary.BreakTransform` (`SceneComponent.K2_GetComponentToWorld` (`self.Arrow_0`))))
  (bind _returnvalue (`|SpawnActorFromClass` "/Game/Blueprints/Weapons/AbilityActors/PTT_Shield.PTT_Shield_C" (`KismetMathLibrary.MakeTransform` _returnvalue_location) "AlwaysSpawn" "MultiplyWithRoot" self 1.0 300.0 300.0 false 1.0 self true 500.0 null))
  (`self.K2_AttachToComponent` _returnvalue (`self.Arrow_0`) "None" "SnapToTarget" "SnapToTarget" "KeepWorld" true))

(event `EnhancedInput|/Game/Input/Ability`
  (params (ActionValue :type Boolean) (ElapsedSeconds :type "Float (double-precision)") (TriggeredSeconds :type "Float (double-precision)") (InputAction :type "InputAction Object Reference" :default "/Game/Input/Ability.Ability"))
  (:`Triggered`
    (if (`self.AllowInput`)
      (if (`self.IsAbilityReady`)
        (set `self.AbilityCharge` 0.0)
        (`/Engine/EditorBlueprintResources/ActorMacros.Switch Has Authority`
          (:`Authority`
            (`self.RPC_UseAbility`))
          (:`Remote`
            (`self.RPC_Server_UseAbility`)))
        (set `self.IsAbilityReady` false)
        (set `self.InAbility` true)))))

(fn `UserConstructionScript`
  (`parent.UserConstructionScript`))