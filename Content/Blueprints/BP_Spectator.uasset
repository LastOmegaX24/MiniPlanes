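; Spectator actor that lets a player spawn into the game when the Lock input fires.
; BeginPlay adds the KBM Enhanced Input mapping context to the Mini_PC controller with ID 0.
; Lock passes that controller through RPC_Server_Spawn to RPC_Spawn, which spawns an actor at a random PlayerStart, has the controller possess it, then destroys the spectator.
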(event `self.ReceiveBeginPlay`
  (bind _asmini_pc (cast `/Game/Blueprints/Mini_PC` (`GameplayStatics.GetPlayerControllerFromID` 0)))
  (`EnhancedInputSubsystemInterface.AddMappingContext` (pcsubsystem `EnhancedInputLocalPlayerSubsystem` _asmini_pc) "/Game/Input/KBM.KBM" 0 (struct)))

(event `EnhancedInput|/Game/Input/Lock`
  (params (ActionValue :type Boolean) (ElapsedSeconds :type "Float (double-precision)") (TriggeredSeconds :type "Float (double-precision)") (InputAction :type "InputAction Object Reference" :default "/Game/Input/Lock.Lock"))
  (:`Started`
    (`self.RPC_Server_Spawn` (`GameplayStatics.GetPlayerControllerFromID` 0))))

(event `RPC_Server_Spawn`
  (params (Target :type "Controller Object Reference"))
  (`self.RPC_Spawn` Target))

(event `RPC_Spawn`
  (params (Target :type "Controller Object Reference"))
  (bind _outactors (`GameplayStatics.GetAllActorsOfClass` "/Script/Engine.PlayerStart"))
  (bind _returnvalue (`|SpawnActorFromClass` (`self.Class`) (`self.GetTransform` (`KismetArrayLibrary.Array_Random` _outactors)) "Undefined" "MultiplyWithRoot" null (struct :`R` 0.109375 :`G` 0.109375 :`B` 0.109375) null))
  (`Controller.Possess` Target _returnvalue)
  (`self.K2_DestroyActor`))

(fn `UserConstructionScript`)