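; Menu pawn for a 3D plane selection screen, where each player claims one of four select platforms and picks an aircraft.
; On restart it adds keyboard/mouse input mapping, creates the selection UI, gathers platforms and claims the first available through RPC-named events.
; Timelines lerp the camera between its menu position and the claimed platform's camera.
; Selections go to the platform and, keyed by Steam ID, to the GameInstance.
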(event `self.ReceiveRestarted`
  (bind _asmini_pc (cast `/Game/Blueprints/Mini_PC` (`GameplayStatics.GetPlayerControllerFromID` 0)))
  (set `self.As Mini PC` _asmini_pc)
  (`EnhancedInputSubsystemInterface.AddMappingContext` (pcsubsystem `EnhancedInputLocalPlayerSubsystem` _asmini_pc) "/Game/Input/KBM.KBM" 0 (struct))
  (`self.RunOnClient`)
  (bind _outactors (`GameplayStatics.GetAllActorsOfClass` "/Game/Blueprints/System/PlayerSelectPlatform.PlayerSelectPlatform_C"))
  (for _array_element _outactors
    (`KismetArrayLibrary.Array_Set` (`self.Out Actors`) (`/Game/Blueprints/System/PlayerSelectPlatform.Index` _array_element) _array_element true))
  (`self.RPC_Server_FindPlatform`))

(event `RunOnClient`
  (bind _returnvalue (`|CreateWidget` "/Game/Menu/SelectPlaneUI.SelectPlaneUI_C" null self (`GameplayStatics.GetPlayerControllerFromID` 0)))
  (`UserWidget.AddToViewport` _returnvalue 0))

(event `RPC_Server_FindPlatform`
  (bind _out_actors (`self.Out Actors`))
  (bind _selectedplatform (`self.SelectedPlatform`))
  (bind _output (`|GetArrayItem` _out_actors 3))
  (bind _output_2 (`|GetArrayItem` _out_actors))
  (bind _output_3 (`|GetArrayItem` _out_actors 1))
  (bind _output_4 (`|GetArrayItem` _out_actors 2))
  (`/Engine/EditorBlueprintResources/StandardMacros.DoOnce` false
    (:`Completed`
      (`/Engine/EditorBlueprintResources/StandardMacros.IsValid` _output_2
        (:`Is Valid`
          (if (`/Game/Blueprints/System/PlayerSelectPlatform.IsAvailable` _output_2)
            (set `self.SelectedPlatform` _output_2)
            (set `self.PlayerIndex` 0)
            (`/Engine/EditorBlueprintResources/StandardMacros.IsValid` _selectedplatform :!label _label
              (:`Is Valid`
                (`/Game/Blueprints/System/PlayerSelectPlatform.ClaimSpawn` _selectedplatform (`GameplayStatics.GetPlayerControllerFromID` 0))
                (`self.RPC_ClaimSpawn`)))
            (elif (`/Game/Blueprints/System/PlayerSelectPlatform.IsAvailable` _output_3)
              (set `self.SelectedPlatform` _output_3)
              (set `self.PlayerIndex` 1)
              (goto _label)
              (elif (`/Game/Blueprints/System/PlayerSelectPlatform.IsAvailable` _output_4)
                (set `self.SelectedPlatform` _output_4)
                (set `self.PlayerIndex` 2)
                (goto _label)
                (elif (`/Game/Blueprints/System/PlayerSelectPlatform.IsAvailable` _output)
                  (set `self.SelectedPlatform` _output)
                  (set `self.PlayerIndex` 3)
                  (goto _label))))))))))

(event `/Game/Blueprints/Interface/ZoomInOut.ZoomIn`
  (bind _selectedplatform (`self.SelectedPlatform`))
  (`/Engine/EditorBlueprintResources/StandardMacros.IsValid` _selectedplatform
    (:`Is Valid`
      (set `self.OriginalCamPos_2` (`SceneComponent.K2_GetComponentToWorld` (`self.Camera`)))
      (bind (_direction _newtrack_0) (`Timeline|Zoom` :!via `PlayFromStart`)
        (:`Update`
          (`SceneComponent.K2_SetWorldTransform` (`self.Camera`) (`KismetMathLibrary.TLerp` (`self.OriginalCamPos_2`) (`SceneComponent.K2_GetComponentToWorld` (`/Game/Blueprints/System/PlayerSelectPlatform.Camera` _selectedplatform)) _newtrack_0) false false))))))

(event `RPC_ClaimSpawn`
  (`SceneComponent.SetVisibility` (`/Game/Blueprints/System/PlayerSelectPlatform.Loading` (`self.SelectedPlatform`)) true false))

(event `/Game/Blueprints/Interface/ZoomInOut.ZoomOut`
  (set `self.MovedCamPos` (`SceneComponent.GetRelativeTransform` (`self.Camera`)))
  (bind (_direction _newtrack_0) (`Timeline|ZoomOutT` :!via `PlayFromStart`)
    (:`Update`
      (`SceneComponent.K2_SetRelativeTransform` (`self.Camera`) (`KismetMathLibrary.TLerp` (`self.MovedCamPos`) (`self.OriginalCamPos`) _newtrack_0) false false))))

(event `/Game/Blueprints/Interface/SelectedAircraft.SendSelect`
  (params (Option :type "/Game/Blueprints/BP_MiniAircraft Class Reference"))
  (bind _output_get (set `self.SelectedPlane` Option))
  (`self.RPC_SendSelect` (`self.SelectedPlatform`) _output_get))

(event `RPC_SendSelect`
  (params (Target :type "Object Object Reference") (Option :type "/Game/Blueprints/BP_MiniAircraft Class Reference"))
  (message `/Game/Blueprints/Interface/SelectedAircraft.SendSelect` Target Option)
  (bind _returnvalue (`SteamProUser.GetSteamID`))
  (message `/Game/Blueprints/Interface/SendAllPlayerData.SendData` (`GameplayStatics.GetGameInstance`) (make `/Game/MapData/PlayerDataStruct` (`GameplayStatics.GetPlayerControllerFromID` 0) (`self.SelectedPlane`)) _returnvalue))

(fn `UserConstructionScript`)