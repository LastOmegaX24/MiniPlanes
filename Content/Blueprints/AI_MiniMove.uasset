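; GMC movement component for an AI mini aircraft that steers toward a random point near player 0, re-picked after two-second delays.
; Each prediction tick yaws toward that point, bleeds speed in turns, moves forward around a set flight height, explodes below half stall speed and tilts the mesh cosmetically.
; Stats come from a data table; input events drive throttle, afterburner and a Cobra maneuver.
; Movement state is bound for GMC replication.
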(event `self.ReceiveBeginPlay`
  (bind _asai_mini_aircraft (cast `/Game/Blueprints/AI_MiniAircraft` (`self.GetGMCPawnOwner`)))
  (bind _output_get (set `self.As BP Mini Aircraft` _asai_mini_aircraft))
  (bind _returnvalue (`|GetDataTableRow` (`self.StatDataTable`) (`/Game/Blueprints/Aircraft.AircraftName` _output_get))
    (:`then`
      (bind _output_get_2 (set `self.AircraftData` _returnvalue))
      (bind (_maxthrust _maxspeed _minspeedstall _acceleration _brakespeed) (break `/Game/AircraftData/AircraftDataStructure` _output_get_2))
      (set `self.Acceleration` _acceleration)
      (set `self.BrakeSpeed` _brakespeed)
      (set `self.MaxThrust` _maxthrust)
      (bind _asgmc_player_controller (cast `GMC_PlayerController` (`GameplayStatics.GetPlayerControllerFromID` 0)))
      (set `self.As GMC Player Controller` _asgmc_player_controller)
      (`EnhancedInputSubsystemInterface.AddMappingContext` (pcsubsystem `EnhancedInputLocalPlayerSubsystem` _asgmc_player_controller) "/Game/Input/KBM.KBM" 0 (struct)))))

(event `self.GenPredictionTick`
  (params (DeltaTime :type "Float (single-precision)"))
  (`self.RotateToPointer`)
  (`self.TurnSlow`)
  (`self.Move` DeltaTime)
  (`self.CosmeticTurn`))

(event `EnhancedInput|/Game/Input/Cobra`
  (params (ActionValue :type Boolean) (ElapsedSeconds :type "Float (double-precision)") (TriggeredSeconds :type "Float (double-precision)") (InputAction :type "InputAction Object Reference" :default "/Game/Input/Cobra.Cobra"))
  (bind (_maxthrust _maxspeed _minspeedstall _acceleration _brakespeed) (break `/Game/AircraftData/AircraftDataStructure` (`self.AircraftData`)))
  (:`Triggered`
    (if (`.CanCobra_73_30CB66824479156A7B17A49E7E422F9B` (break `/Game/AircraftData/AircraftDataStructure` (`self.AircraftData`)))
      (if (and (`self.CobraReady`) (< (`self.CurrentSpeed`) 800.0))
        (set `self.IsCobra` true)
        (set `self.BlockThrottleInput` true)
        (set `self.TargetThrust` 0.0)
        (set `self.BrakeSpeed` 100.0)
        (`KismetSystemLibrary.Delay` 1.2)
        (set `self.CobraRecover` true)
        (`KismetSystemLibrary.Delay` 1.0)
        (set `self.BlockThrottleInput` false)
        (set `self.IsCobra` false)
        (set `self.CobraRecover` false)
        (set `self.BrakeSpeed` _brakespeed)
        (set `self.TargetThrust` _minspeedstall)
        (`KismetSystemLibrary.Delay` 10.0)
        (set `self.CobraReady` true)))))

(event `self.ReceiveTick`
  (params (DeltaSeconds :type "Float (single-precision)"))
  (bind _x (.x (`Actor.K2_GetActorLocation` (`GameplayStatics.GetPlayerPawn` 0))))
  (bind _y (.y (`Actor.K2_GetActorLocation` (`GameplayStatics.GetPlayerPawn` 0))))
  (`KismetSystemLibrary.Delay` 2.0)
  (if (`/Game/Blueprints/Aircraft.AllowInput` (`self.As BP Mini Aircraft`))
    (set `self.Impact Point` (`KismetMathLibrary.MakeVector` (`KismetMathLibrary.RandomFloatInRange` (- _x 1000.0) (+ _x 1000.0)) (`KismetMathLibrary.RandomFloatInRange` (- _y 1000.0) (+ _y 1000.0))))))

(event `EnhancedInput|/Game/Input/Afterburner`
  (params (ActionValue :type Boolean) (ElapsedSeconds :type "Float (double-precision)") (TriggeredSeconds :type "Float (double-precision)") (InputAction :type "InputAction Object Reference" :default "/Game/Input/Afterburner.Afterburner"))
  (bind (_maxthrust _maxspeed _minspeedstall _acceleration) (break `/Game/AircraftData/AircraftDataStructure` (`self.AircraftData`)))
  (bind _returnvalue (* _maxthrust 1.3))
  (:`Triggered`
    (if (not (`self.BlockThrottleInput`))
      (set `self.TargetThrust` _returnvalue)
      (set `self.MaxThrust` _returnvalue)
      (set `self.Acceleration` (* _acceleration 4.0))
      (set `self.IsAfterburner` true)))
  (:`Canceled`
    (if (not (`self.BlockThrottleInput`)) :!label _label
      (set `self.TargetThrust` _maxthrust)
      (set `self.MaxThrust` _maxthrust)
      (set `self.Acceleration` _acceleration)
      (set `self.IsAfterburner` false)))
  (:`Completed`
    (goto _label)))

(event `Takeoff`)

(event `self.BindReplicationData`
  (`parent.BindReplicationData`)
  (`self.BindDoublePrecisionFloat` (`self.TargetThrust`) "ClientAuth_Input" "CombineIfUnchanged" "Periodic_Output" "NearestNeighbour")
  (`self.BindCompressedVector` (`self.Impact Point`) "ClientAuth_Input" "AlwaysCombine" "PeriodicAndOnChange_Output" "NearestNeighbour")
  (`self.BindDoublePrecisionFloat` (`self.MaxThrust`) "ClientAuth_Input" "CombineIfUnchanged" "Periodic_Output" "NearestNeighbour")
  (`self.BindActorReference` (`self.As GMC Player Controller`) "ClientAuth_Input" "AlwaysCombine" "Periodic_Output" "NearestNeighbour")
  (`self.BindDoublePrecisionFloat` (`self.CurrentSpeed`) "ServerAuth_InputOutput_ServerValidated" "AlwaysCombine" "Periodic_Output" "NearestNeighbour")
  (`self.BindDoublePrecisionFloat` (`self.CurrentSpeed`) "ServerAuth_InputOutput_ServerValidated" "AlwaysCombine" "Periodic_Output" "NearestNeighbour")
  (`self.BindCompressedRotator` (`self.TargetRot`) "ClientAuth_Input" "AlwaysCombine" "None" "NearestNeighbour")
  (`self.BindCompressedRotator` (`self.CurrentRot`) "ServerAuth_Output_ClientValidated" "CombineIfUnchanged" "Periodic_InputOutput" "NearestNeighbour")
  (`self.BindBool` (`self.IsCobra`) "ClientAuth_Input" "AlwaysCombine" "Periodic_Output" "NearestNeighbour")
  (`self.BindBool` (`self.IsAfterburner`) "ClientAuth_Input" "AlwaysCombine" "Periodic_Output" "NearestNeighbour")
  (`self.BindBool` (`self.CobraRecover`) "ClientAuth_Input" "AlwaysCombine" "Periodic_Output" "NearestNeighbour")
  (`self.BindDoublePrecisionFloat` (`self.Acceleration`) "ServerAuth_InputOutput_ClientValidated" "AlwaysCombine" "Periodic_Output" "NearestNeighbour")
  (`self.BindDoublePrecisionFloat` (`self.BrakeSpeed`) "ServerAuth_InputOutput_ClientValidated" "AlwaysCombine" "Periodic_Output" "NearestNeighbour")
  (`self.BindDoublePrecisionFloat` (`self.FlightAngle`) "ServerAuth_InputOutput_ServerValidated" "CombineIfUnchanged" "Periodic_Output" "NearestNeighbour"))

(event `EnhancedInput|/Game/Input/Thrust`
  (params (ActionValue :type "Float (double-precision)") (ElapsedSeconds :type "Float (double-precision)") (TriggeredSeconds :type "Float (double-precision)") (InputAction :type "InputAction Object Reference" :default "/Game/Input/Thrust.Thrust"))
  (bind (_maxthrust _maxspeed _minspeedstall) (break `/Game/AircraftData/AircraftDataStructure` (`self.AircraftData`)))
  (:`Triggered`
    (if (not (`self.BlockThrottleInput`))
      (set `self.TargetThrust` (`KismetMathLibrary.FClamp` (+ (`self.TargetThrust`) (* (`self.ThrustSens`) (`self.GetPhysDeltaTime`) ActionValue)) _minspeedstall _maxthrust)))))

(event `EnhancedInput|/Game/Input/Scroll`
  (params (ActionValue :type "Float (double-precision)") (ElapsedSeconds :type "Float (double-precision)") (TriggeredSeconds :type "Float (double-precision)") (InputAction :type "InputAction Object Reference" :default "/Game/Input/Scroll.Scroll")))

(fn `CosmeticTurn`
  (if (`self.IsCobra`)
    (bind _as_bp_mini_aircraft (`self.As BP Mini Aircraft`)
      (:`then`
        (bind _planemesh (`/Game/Blueprints/Aircraft.PlaneMesh` _as_bp_mini_aircraft))
        (bind _returnvalue_roll (`KismetMathLibrary.BreakRotator` (`SceneComponent.GetSocketRotation` _planemesh "None")))
        (`SceneComponent.K2_SetRelativeRotation` _planemesh (`KismetMathLibrary.MakeRotator` (`KismetMathLibrary.Lerp` _returnvalue_roll (`KismetMathLibrary.SelectFloat` 0.0 -105.0 (`self.CobraRecover`)) 0.05)) false true))
      (:`else`))
    (else
      (bind _as_bp_mini_aircraft_2 (`self.As BP Mini Aircraft`)
        (:`then`
          (bind _planemesh_2 (`/Game/Blueprints/Aircraft.PlaneMesh` _as_bp_mini_aircraft_2))
          (bind (_returnvalue_roll_2 _returnvalue_pitch _returnvalue_yaw) (`KismetMathLibrary.BreakRotator` (`KismetMathLibrary.RLerp` (`SceneComponent.GetSocketRotation` _planemesh_2 "None") (`KismetMathLibrary.MakeRotator` (- (.roll (`self.TargetRot`)) (.roll (`self.GetRootCollisionRotation`))) (- (.pitch (`self.TargetRot`)) (.pitch (`self.GetRootCollisionRotation`))) (- (.yaw (`self.TargetRot`)) (.yaw (`self.GetRootCollisionRotation`)))) 1.0 true)))
          (`SceneComponent.K2_SetRelativeRotation` _planemesh_2 (`KismetMathLibrary.MakeRotator` (`KismetMathLibrary.Lerp` (.roll (`SceneComponent.GetSocketRotation` _planemesh_2 "None")) (`KismetMathLibrary.FClamp` (`self.FlightAngle`) -35.0 35.0) 0.1) (`KismetMathLibrary.FClamp` _returnvalue_yaw -80.0 80.0)) false true))
        (:`else`)))))

(fn `Move`
  (params (DeltaTime :type "Float (single-precision)"))
  (bind _flightheight (`self.FlightHeight`))
  (bind _z (.z (`self.GetActorLocation_GMC`)))
  (bind (_returnvalue_roll _returnvalue_pitch) (`KismetMathLibrary.BreakRotator` (`KismetMathLibrary.FindLookAtRotation` (`KismetMathLibrary.MakeVector` 0.0 0.0 _flightheight) (`KismetMathLibrary.MakeVector` 0.0 0.0 _z))))
  (bind _output_get (set `self.CurrentSpeed` (`KismetMathLibrary.SelectFloat` (`KismetMathLibrary.FInterpTo_Constant` (`self.CurrentSpeed`) (`self.TargetThrust`) DeltaTime (`self.Acceleration`)) (`KismetMathLibrary.FInterpTo_Constant` (`self.CurrentSpeed`) (`self.TargetThrust`) DeltaTime (`self.BrakeSpeed`)) (< (`self.CurrentSpeed`) (`self.TargetThrust`)))))
  (if (> _output_get (/ (`.MinSpeedStall_8_870E7CA74FE69C2E1EB2CB83235D7E89` (break `/Game/AircraftData/AircraftDataStructure` (`self.AircraftData`))) 2.0))
    (`self.UpdateVelocity` (* (`self.CurrentSpeed`) (`Actor.GetActorForwardVector` (`self.GetGMCPawnOwner`)) (`self.SpeedMultiplier`)) DeltaTime)
    (`/Engine/EditorBlueprintResources/StandardMacros.CompareFloat` _z _flightheight
      (:`>`
        (`self.AddVelocity` (`KismetMathLibrary.MakeVector` 0.0 0.0 -1000.0) DeltaTime))
      (:`==`
        _)
      (:`<`
        (`self.AddVelocity` (`KismetMathLibrary.MakeVector` 0.0 0.0 500.0) DeltaTime)))
    (set `self.FlightAngle` _returnvalue_pitch)
    (`self.K2_MoveUpdatedComponent` (* (`self.GetVelocity`) DeltaTime) (`self.GetRootCollisionRotation`))
    (else
      (`/Engine/EditorBlueprintResources/StandardMacros.DoOnce` false
        (:`Completed`
          (`/Game/Blueprints/BP_MiniAircraft.RPC_Server_Explode` (`self.As BP Mini Aircraft`) false))))))

(fn `RotateToPointer`
  (bind _output_get (set `self.TargetRot` (`KismetMathLibrary.SelectRotator` (`self.CurrentRot`) (`KismetMathLibrary.FindLookAtRotation` (`self.GetRootCollisionLocation`) (`self.Impact Point`)) (`self.IsCobra`))))
  (bind _output_get_2 (set `self.CurrentRot` (`KismetMathLibrary.MakeRotator` 0.0 0.0 (.yaw (`KismetMathLibrary.RLerp` (`self.GetRootCollisionRotation`) _output_get (`KismetMathLibrary.SafeDivide` (`CurveFloat.GetFloatValue` (`.Turnspeed_17_FF247B81499497AE758C9C960762844A` (break `/Game/AircraftData/AircraftDataStructure` (`self.AircraftData`))) (`self.CurrentSpeed`)) (+ (/ (`KismetMathLibrary.Abs` (- (.yaw (`self.TargetRot`)) (.yaw (`self.GetRootCollisionRotation`)))) 90.0) 1.0)) true)))))
  (`Actor.K2_SetActorRotation` (`self.GetPawnOwner`) _output_get_2 false))

(fn `TurnSlow`
  (set `self.CurrentSpeed` (`KismetMathLibrary.FClamp` (- (`self.CurrentSpeed`) (`CurveFloat.GetFloatValue` (`.RateSpeed_24_176D276F417AE96FF01A18B9DE8B46F6` (break `/Game/AircraftData/AircraftDataStructure` (`self.AircraftData`))) (`KismetMathLibrary.Abs` (/ (- (.yaw (`self.TargetRot`)) (.yaw (`self.GetRootCollisionRotation`))) 180.0)))) 0.0 (`self.MaxThrust`))))