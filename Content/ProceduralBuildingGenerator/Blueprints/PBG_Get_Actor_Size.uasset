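; An editor helper actor from the procedural building generator that measures a referenced actor's size and pivot offset.
; Its construction script temporarily zeroes the actor's rotation so the bounds are unrotated, then restores it.
; It stores the full size and the XY shift from bounds center to actor location, and fits a box component to those bounds.
; Flags control whether non-colliding components and child actors count.
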(fn `UserConstructionScript`
  (locals (`Safe Rotation` :type "Rotator Structure"))
  (bind (_origin _boxextent) (`self.GetActorBounds` (`self.Actor`) (`self.Only Colliding Components`) (`self.Include Child Actors`)))
  (bind (_returnvalue_x _returnvalue_y) (`KismetMathLibrary.BreakVector` (- (`self.K2_GetActorLocation` (`self.Actor`)) _origin)))
  (`self.Actor`
    (:`then`
      (set `local.Safe Rotation` (`self.K2_GetActorRotation` (`self.Actor`)))
      (`self.K2_SetActorRotation` :`self` (`self.Actor`))
      (set `self.Origin Shift` (`KismetMathLibrary.MakeVector` _returnvalue_x _returnvalue_y))
      (set `self.Actor Size` _boxextent)
      (`BoxComponent.SetBoxExtent` (`self.Box`) (`self.Actor Size`) true)
      (`SceneComponent.K2_SetWorldLocation` (`self.Box`) _origin false false)
      (set `self.Actor Size` (* (`self.Actor Size`) 2))
      (`self.K2_SetActorRotation` (`self.Actor`) (`local.Safe Rotation`) false))
    (:`else`)))