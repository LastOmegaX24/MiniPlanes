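; Aircraft pawn that loads its stats from a data table and handles health, shields, weapons, radar locking and crashing.
; Each tick it emits AI noise scaled by radar cross-section until crashing.
; Radar builds per-target lock from power, distance and RCS within a dot-product cone, while a box trace cycles the lock target fed to missiles.
; Lethal damage triggers a one-time burning explosion that hides the health bar and removes radar-tagged attachments.
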(event `self.ReceiveBeginPlay`
  (bind (_maxthrust _maxspeed _minspeedstall _acceleration _brakespeed _turnspeed _ratespeed _maxhealth _maxammo _reservemissiles _reloadtime _rcs _gunaccuracy _gundamage _mesh _missilecooldown _radarcone _radarpower _class _skins _fireinterval _cancobra _flarecount) (break `/Game/AircraftData/AircraftDataStructure` (`self.AircraftData`)))
  (message `/Game/Blueprints/Interface/SendPlayerData.SendOwningPawn` (`WidgetComponent.GetWidget` (`self.HealthBar`)) self)
  (bind _returnvalue (`|GetDataTableRow` (`self.StatDataTable`) (`self.AircraftName`))
    (:`then`
      (set `self.AircraftData` _returnvalue)
      (set `self.Health` _maxhealth)
      (bind _output_get (set `self.MaxMissileIndex` _reservemissiles))
      (set `self.MissileCount` _output_get)
      (set `self.FlareCount` _flarecount)
      (`self.RealizeAmmo`))))

(event `self.ReceiveTick`
  (params (DeltaSeconds :type "Float (single-precision)"))
  (if (not (`self.Crashing`))
    (`PawnNoiseEmitterComponent.MakeNoise` (`self.PawnNoiseEmitter`) self (`.RCS_41_FD4138704F1C607D4A1BFE9F573CC7BC` (break `/Game/AircraftData/AircraftDataStructure` (`self.AircraftData`))) (`self.K2_GetActorLocation`))))

(event `self.ReceiveAnyDamage`
  (params (Damage :type "Float (single-precision)") (DamageType :type "DamageType Object Reference") (InstigatedBy :type "Controller Object Reference") (DamageCauser :type "Actor Object Reference"))
  (set `self.Instigated By` InstigatedBy)
  (set `self.Damage Causer` DamageCauser)
  (bind _output_get (set `self.Health` (- (`self.Health`) Damage)))
  (if (<= _output_get 0.0)
    (`/Engine/EditorBlueprintResources/StandardMacros.DoOnce` false
      (:`Completed`
        (`|ExecutionSequence`
          (:`then_0`
            (`self.RPC_Explode` true)))))))

(event `Heal`
  (params (HealFrom :type "Actor Object Reference") (Amount :type "Float (double-precision)"))
  (set `self.Health` (`KismetMathLibrary.FClamp` (+ (`self.Health`) Amount) 0.0 (`.MaxHealth_27_C0B3CFFF4C07100E5FA2C6BA75517302` (break `/Game/AircraftData/AircraftDataStructure` (`self.AircraftData`))))))

(event `AddShield`
  (params (HP :type "Float (double-precision)") (`Max HP` :type "Float (double-precision)") (Radius :type "Float (double-precision)") (Regenerate :type Boolean) (Parent :type "/Game/Blueprints/Aircraft Object Reference") (DestroyIfDisabled :type Boolean) (ActivationThreshhold :type "Float (double-precision)") (RegenRate :type "Float (double-precision)"))
  (bind _returnvalue_location (`KismetMathLibrary.BreakTransform` (`SceneComponent.K2_GetComponentToWorld` (`self.SpawnArrow`))))
  (bind _returnvalue (`|SpawnActorFromClass` "/Game/Blueprints/Weapons/Shield.Shield_C" (`KismetMathLibrary.MakeTransform` _returnvalue_location) "AlwaysSpawn" "MultiplyWithRoot" null Radius HP `Max HP` Regenerate RegenRate Parent DestroyIfDisabled ActivationThreshhold null))
  (`self.K2_AttachToComponent` _returnvalue (`self.SpawnArrow`) "None" "KeepRelative" "KeepRelative" "KeepRelative" true))

(event `RPC_Server_Explode`
  (params (Burning :type Boolean))
  (`self.RPC_Explode` Burning))

(event `RPC_Explode`
  (params (Burning :type Boolean))
  (set `self.Crashing` true)
  (`SceneComponent.SetVisibility` (`self.HealthBar`) false false)
  (if Burning
    (`GameplayStatics.SpawnEmitterAttached` "/Engine/Tutorial/SubEditors/TutorialAssets/TutorialParticleSystem.TutorialParticleSystem" (`self.PlaneMesh`) "None" (0.0 0.0 0.0) (struct) (2.0 2.0 2.0)))
  (for _array_element (`self.GetAttachedActors` true)
    (if (`self.ActorHasTag` _array_element "rdr")
      (`self.K2_DestroyActor` _array_element))))

(event `/Game/Blueprints/Interface/AbilityStatus.AbilityEnded`
  (set `self.InAbility` false))

(event `/Game/Blueprints/Interface/AbilityStatus.AbilityStarted`
  (set `self.InAbility` true))

(fn `CreateThruster`
  (params (Target :type "Array of PrimitiveComponent Object Reference") (bPickA :type Boolean))
  (bind _returnvalue (`KismetMathLibrary.SelectFloat` 1.0 0.0 bPickA))
  (for _array_element Target
    (`/Engine/EditorBlueprintResources/StandardMacros.IsValid` _array_element
      (:`Is Valid`
        (bind _returnvalue_2 (`PrimitiveComponent.CreateDynamicMaterialInstance` _array_element 0 (`PrimitiveComponent.GetMaterial` _array_element 0) "None"))
        (`MaterialInstanceDynamic.SetScalarParameterValue` _returnvalue_2 "Thrust" _returnvalue)
        (`PrimitiveComponent.SetMaterial` _array_element 0 _returnvalue_2)
        (bind _returnvalue_3 (`PrimitiveComponent.CreateDynamicMaterialInstance` _array_element 1 (`PrimitiveComponent.GetMaterial` _array_element 1) "None"))
        (`MaterialInstanceDynamic.SetScalarParameterValue` _returnvalue_3 "Thrust" _returnvalue)
        (`PrimitiveComponent.SetMaterial` _array_element 1 _returnvalue_3)))))

(fn `LockTargetStart`
  (bind _targetlocktracker (`self.TargetLockTracker`))
  (bind _gun (`self.Gun`))
  (bind _locktarget (`self.LockTarget`))
  (bind _ignorelock (`self.IgnoreLock`))
  (bind _returnvalue (`SceneComponent.K2_GetComponentLocation` _gun))
  (bind _returnvalue_2 (`SceneComponent.K2_GetComponentRotation` _gun))
  (`/Engine/EditorBlueprintResources/StandardMacros.IsValid` _locktarget
    (:`Is Valid`
      (`KismetArrayLibrary.Array_Add` _ignorelock _locktarget))
    (:`Is Not Valid`
      (`KismetArrayLibrary.Array_Clear` _ignorelock)))
  (bind (_outhits _returnvalue_3) (`KismetSystemLibrary.BoxTraceMultiForObjects` _returnvalue (+ _returnvalue (* (`KismetMathLibrary.GetForwardVector` _returnvalue_2) (`self.RadarMaxRange`))) (`self.RadarRangeVec3D`) _returnvalue_2 (`|MakeArray` "ObjectTypeQuery3" :!type "EObjectTypeQuery Enum") false (`self.IgnoreLock`)))
  (for _array_element _outhits
    _)
  (if (not _returnvalue_3)
    (`KismetArrayLibrary.Array_Clear` (`self.IgnoreLock`)))
  (bind (_bblockinghit _binitialoverlap _time _distance _location _impactpoint _normal _impactnormal _physmat _hitactor) (`GameplayStatics.BreakHitResult` _array_element))
  (`/Engine/EditorBlueprintResources/StandardMacros.IsValid` _hitactor
    (:`Is Valid`
      (set `self.Location` _location)
      (bind _output_get (set `self.LockTarget` _hitactor))
      (`/Engine/EditorBlueprintResources/StandardMacros.IsValid` _output_get
        (:`Is Valid`
          _)
        (:`Is Not Valid`
          (`self.K2_DestroyActor` _targetlocktracker)))
      (`/Engine/EditorBlueprintResources/StandardMacros.IsValid` _targetlocktracker
        (:`Is Valid`
          (`/Game/Blueprints/Target_Lock.ReCast` _targetlocktracker))
        (:`Is Not Valid`
          (bind _returnvalue_4 (`|SpawnActorFromClass` "/Game/Blueprints/Target_Lock.Target_Lock_C" (`KismetMathLibrary.MakeTransform` (0.0 0.0 0.0)) "AlwaysSpawn" "OverrideRootScale" (`GameplayStatics.GetPlayerPawn` 0) self null))
          (`self.SetActorHiddenInGame` _returnvalue_4 false)
          (bind _output_get_2 (set `self.TargetLockTracker` _returnvalue_4))
          (message `/Game/Blueprints/Interface/LockSendData.SendLock` (`WidgetComponent.GetWidget` (`/Game/Blueprints/Target_Lock.Widget` _output_get_2)) _output_get_2))))))

(fn `OnRep_CanFlare`)

(fn `RadarProgressV2`
  (params (InputObject :type "Actor Object Reference") (RCS :type "Float (double-precision)"))
  (bind _returnvalue (`KismetArrayLibrary.Array_Find` (`self.AlreadyTrackingProg`) InputObject))
  (bind _output (`|GetArrayItem` (`self.TargetProg`) _returnvalue))
  (`/Engine/EditorBlueprintResources/StandardMacros.IsValid` InputObject
    (:`Is Valid`
      (if (== _returnvalue -1)
        (bind _returnvalue_2 (`|SpawnActorFromClass` "/Game/Blueprints/Target_Prog_Lock.Target_Prog_Lock_C" (`KismetMathLibrary.MakeTransform` (0.0 0.0 0.0)) "AlwaysSpawn" "OverrideRootScale" (`GameplayStatics.GetPlayerPawn` 0) self null))
        (`self.SetActorHiddenInGame` _returnvalue_2 false)
        (bind _returnvalue_3 (`KismetArrayLibrary.Array_Add` (`self.TargetProg`) _returnvalue_2))
        (set `self.LockIndex` _returnvalue_3)
        (`KismetArrayLibrary.Array_Add` (`self.AlreadyTrackingProg`) InputObject)
        (`self.K2_AttachToActor` _returnvalue_2 InputObject "None" "SnapToTarget" "SnapToTarget" "SnapToTarget" false)
        (message `/Game/Blueprints/Interface/LockingRWR.StartLock` self InputObject)
        (else
          (`/Engine/EditorBlueprintResources/StandardMacros.IsValid` _output
            (:`Is Valid`
              (`self.IsInRadarCone` (`self.GetActorForwardVector`) (`self.K2_GetActorLocation`) (`self.K2_GetActorLocation` InputObject) (`.RadarCone_58_F43130EF41F4A47B8FF590B0DC858726` (break `/Game/AircraftData/AircraftDataStructure` (`self.AircraftData`)))
                (:`True`
                  (set `/Game/Blueprints/Target_Prog_Lock.LockProgression` (`KismetMathLibrary.FClamp` (+ (`/Game/Blueprints/Target_Prog_Lock.LockProgression` _output) (`KismetMathLibrary.SafeDivide` (* 100.0 (`.RadarPower_60_D5961DFF43152F11F40B1FB73D82FF32` (break `/Game/AircraftData/AircraftDataStructure` (`self.AircraftData`))) RCS (`GameplayStatics.GetWorldDeltaSeconds`)) (`self.GetDistanceTo` self InputObject)))) _output)
                  (`/Game/Blueprints/Target_Prog_Lock.LoseLockDelay` _output)
                  (message `/Game/Blueprints/Interface/LockingRWR.Locking` InputObject self))))))))))

(fn `RealizeAmmo`
  (bind (_maxthrust _maxspeed _minspeedstall _acceleration _brakespeed _turnspeed _ratespeed _maxhealth _maxammo _reservemissiles) (break `/Game/AircraftData/AircraftDataStructure` (`self.AircraftData`)))
  (set `self.Ammo` _maxammo)
  (set `self.MissileCount` _reservemissiles))

(fn `ShootGunF`
  (params (CanHit :type Boolean) (Accuracy :type "Float (double-precision)") (Damage :type "Float (double-precision)") (ParentPlayer :type "/Game/Blueprints/Aircraft Object Reference") (InitialSpeed :type "Float (double-precision)"))
  (bind _returnvalue (* Accuracy -1.0))
  (if (not (`self.Crashing`))
    (`|SpawnActorFromClass` "/Game/Blueprints/Weapons/Bullet.Bullet_C" (`KismetMathLibrary.MakeTransform` (.location (`SceneComponent.K2_GetComponentToWorld` (`self.Gun`))) (`KismetMathLibrary.MakeRotator` (.roll (.rotation (`SceneComponent.K2_GetComponentToWorld` (`self.Gun`)))) (+ (.pitch (.rotation (`SceneComponent.K2_GetComponentToWorld` (`self.Gun`)))) (`KismetMathLibrary.RandomFloatInRange` Accuracy _returnvalue)) (+ (.yaw (.rotation (`SceneComponent.K2_GetComponentToWorld` (`self.Gun`)))) (`KismetMathLibrary.RandomFloatInRange` Accuracy _returnvalue))) (.scale (`SceneComponent.K2_GetComponentToWorld` (`self.Gun`)))) "AlwaysSpawn" "MultiplyWithRoot" null CanHit Damage (`GameplayStatics.GetPlayerControllerFromID` 0) ParentPlayer InitialSpeed ParentPlayer)))

(fn `ShootMissile`
  (params (InitialSpeed :type "Float (double-precision)"))
  (set `self.MissileIndex` 0)
  (`|SpawnActorFromClass` (`self.MissileClass`) (`KismetMathLibrary.MakeTransform` (.location (`SceneComponent.K2_GetComponentToWorld` (`self.MissileSpecial`))) (.rotation (`SceneComponent.K2_GetComponentToWorld` (`self.MissileSpecial`)))) "AlwaysSpawn" "OverrideRootScale" null (`self.LockTarget`) self InitialSpeed self)
  (`/Engine/EditorBlueprintResources/StandardMacros.DecrementInt` (`self.MissileCount`)))

(fn `UserConstructionScript`)