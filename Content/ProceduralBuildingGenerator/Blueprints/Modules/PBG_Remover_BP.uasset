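; Procedural building generator module that clears roof props inside a box volume.
; Remove Props resizes the box, finds overlapping actors and filters them by the roof props tag.
; Tagged PBG_OptiMesh_BP actors lose only the mesh instances whose locations lie in the box, and are destroyed once empty.
; Other tagged actors, whether static mesh or Blueprint, are destroyed outright.
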(fn `Remove Props`
  (locals (`Instance IDs` :type "Array of Integer") (`ISM Ref` :type "InstancedStaticMeshComponent Object Reference") (`PBG Opti Ref` :type "/Game/ProceduralBuildingGenerator/Blueprints/PBG_OptiMesh_BP Object Reference"))
  (bind _box (`self.Box`))
  (bind _box_2 (`self.Box`))
  (bind (_returnvalue_x _returnvalue_y) (`KismetMathLibrary.BreakVector` (`BoxComponent.GetScaledBoxExtent` _box_2)))
  (`BoxComponent.SetBoxExtent` (`self.Box`) (`self.TBox Extent`) true)
  ;[1 1 1] This will remove any actors with that tag (work for both Static Mesh & BP actors)
  (bind _outactors (`KismetSystemLibrary.ComponentOverlapActors` _box (`SceneComponent.K2_GetComponentToWorld` _box) (`self.Object Types`) "/Script/Engine.Actor"))
  (for _array_element _outactors
    (`KismetArrayLibrary.Array_Clear` (`local.Instance IDs`))
    (if (`self.ActorHasTag` _array_element (`self.Roof Props Tag`))
      (bind _aspbg_opti_mesh_bp (cast `/Game/ProceduralBuildingGenerator/Blueprints/PBG_OptiMesh_BP` _array_element)
        (:`then`
          (bind _output_get (set `local.PBG Opti Ref` _aspbg_opti_mesh_bp))
          (set `local.ISM Ref` (`/Game/ProceduralBuildingGenerator/Blueprints/PBG_OptiMesh_BP.InstancedStaticMesh` _output_get))
          ;[1 1 1] Remove Instanced Components
          (for _index (range (`InstancedStaticMeshComponent.GetInstanceCount` (`local.ISM Ref`)))
            (if (`KismetMathLibrary.IsPointInBoxWithTransform` (.location (`InstancedStaticMeshComponent.GetInstanceTransform` (`local.ISM Ref`) _index true)) (`SceneComponent.K2_GetComponentToWorld` _box_2) (`KismetMathLibrary.MakeVector` _returnvalue_x _returnvalue_y (`self.Box Extent Z`)))
              (`KismetArrayLibrary.Array_Add` (`local.Instance IDs`) _index)))
          (if (`KismetArrayLibrary.Array_IsNotEmpty` (`local.Instance IDs`))
            (`InstancedStaticMeshComponent.RemoveInstances` (`local.ISM Ref`) (`local.Instance IDs`)))
          (if (<= (`InstancedStaticMeshComponent.GetInstanceCount` (`local.ISM Ref`)) 0)
            (`self.K2_DestroyActor` (`local.PBG Opti Ref`))))
        (:`CastFailed`
          (`self.K2_DestroyActor` _array_element))))))

(fn `UserConstructionScript`
  (set `self.SpriteScale` (`self.Sprite Scale`)))