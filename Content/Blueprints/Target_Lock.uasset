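; Target lock marker actor that attaches to the owning player's LockTarget and gates that player's ability to track it.
; BeginPlay and ReCast record the target, attach to it and pass the marker and player to its widget.
; Tick sets Locked from full progression on sibling Target_Prog_Lock actors, destroying itself if player or parent is invalid.
; Locked's RepNotify copies the state to the player's CanTrack.
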(event `self.ReceiveBeginPlay`
  (bind _playerref (`self.PlayerRef`))
  (bind _returnvalue (`WidgetComponent.GetWidget` (`self.Widget`)))
  (bind _locktarget (`/Game/Blueprints/BP_MiniAircraft.LockTarget` _playerref))
  (`/Engine/EditorBlueprintResources/StandardMacros.IsValid` _playerref :!label _label
    (:`Is Valid`
      (`KismetArrayLibrary.Array_AddUnique` (`self.Lock Target Arr`) _locktarget)
      (`self.K2_AttachToActor` _locktarget "None" "KeepRelative" "KeepRelative" "KeepRelative" false)
      (message `/Game/Blueprints/Interface/LockSendData.SendLock` _returnvalue self)
      (message `/Game/Blueprints/Interface/SendPlayerData.SendOwningPawn` _returnvalue (`self.PlayerRef`)))))

(event `ReCast`
  (goto _label))

(event `self.ReceiveTick`
  (params (DeltaSeconds :type "Float (single-precision)"))
  (`/Engine/EditorBlueprintResources/StandardMacros.IsValid` (`self.PlayerRef`)
    (:`Is Valid`
      (`/Engine/EditorBlueprintResources/StandardMacros.IsValid` (`self.GetAttachParentActor`)
        (:`Is Valid`
          (for _array_element (`self.GetAttachedActors` (`self.GetAttachParentActor`) true false)
            (bind _astarget_prog_lock (cast `/Game/Blueprints/Target_Prog_Lock` _array_element))
            (set `self.Locked` (== (`/Game/Blueprints/Target_Prog_Lock.LockProgression` _astarget_prog_lock) 1.0))))
        (:`Is Not Valid`
          (`self.K2_DestroyActor`))))
    (:`Is Not Valid`
      (`self.K2_DestroyActor`))))

(fn `OnRep_Locked`
  (bind _playerref (`self.PlayerRef`)
    (:`then`
      (set `/Game/Blueprints/BP_MiniAircraft.CanTrack` (`self.Locked`) _playerref))
    (:`else`)))

(fn `UserConstructionScript`)