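; Projectile actor for a bullet that deals player-type damage to what it overlaps and then destroys itself.
; Box overlaps skip the parent player and other bullets, and only bullets with CanHit set call the server damage RPC, which credits the stored controller.
; The construction script adds a fixed boost to the initial speed and shows the cube mesh only when CanHit is true.
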(event `RPC_Server_Damage`
  (params (DamagedActor :type "Actor Object Reference"))
  (bind _controller (`self.Controller`))
  (`GameplayStatics.ApplyDamage` DamagedActor (`self.Damage`) _controller _controller "/Game/Blueprints/DamageType/PlayerDamage.PlayerDamage_C")
  (`self.K2_DestroyActor`))

(event `self.Box.OnComponentBeginOverlap`
  (params (OverlappedComponent :type "PrimitiveComponent Object Reference") (OtherActor :type "Actor Object Reference") (OtherComp :type "PrimitiveComponent Object Reference") (OtherBodyIndex :type Integer) (bFromSweep :type Boolean) (SweepResult :type "HitResult Structure (by ref)"))
  (if (!= OtherActor (`self.ParentPlayer`))
    (if (!= (`GameplayStatics.GetObjectClass` OtherActor) "Bullet_C")
      (if (`self.CanHit`)
        (`self.RPC_Server_Damage` OtherActor)))))

(fn `UserConstructionScript`
  (set `ProjectileMovementComponent.InitialSpeed` (+ (`self.InitialSpeed`) 1500.0) (`self.ProjectileMovement`))
  (`SceneComponent.SetVisibility` (`self.Cube`) (`self.CanHit`) false))