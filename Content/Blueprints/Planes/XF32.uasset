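; XF32 is a plane Blueprint extending a parent aircraft class, with a hitscan laser as its gun.
; BeginPlay applies the plane color texture through a dynamic material, and Tick updates two thrusters from the afterburner state.
; Its shoot override multi-traces forward from the gun, spawns a laser effect along that line and damages every hit actor using the aircraft data's gun damage, always instigated by player controller 0.
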(event `self.ReceiveBeginPlay`
  (bind _planemesh (`self.PlaneMesh`))
  (`parent.ReceiveBeginPlay`)
  (bind _returnvalue (`PrimitiveComponent.CreateDynamicMaterialInstance` _planemesh 0 (`PrimitiveComponent.GetMaterial` _planemesh 0) "None"))
  (`MaterialInstanceDynamic.SetTextureParameterValue` _returnvalue "txt" (`self.PlaneColor`))
  (`PrimitiveComponent.SetMaterial` _planemesh 0 _returnvalue))

(event `self.ReceiveTick`
  (params (DeltaSeconds :type "Float (single-precision)"))
  (`parent.ReceiveTick` DeltaSeconds)
  (`self.CreateThruster` (`|MakeArray` (`self.StaticMesh1`) (`self.StaticMesh2`) :!type "PrimitiveComponent Object Reference") (`/Game/Blueprints/MiniMove.IsAfterburner` (`self.MiniMove`))))

(event `self.OVR_ShootAll`
  (params (ParentPlayer :type "/Game/Blueprints/BP_MiniAircraft Object Reference"))
  (bind _returnvalue (`SceneComponent.K2_GetComponentLocation` (`self.Gun`)))
  (bind _returnvalue_2 (* (`self.GetActorForwardVector`) 5000.0))
  (bind _outhits (`KismetSystemLibrary.LineTraceMultiForObjects` _returnvalue (+ _returnvalue _returnvalue_2) (`|MakeArray` "ObjectTypeQuery3" "ObjectTypeQuery2" :!type "EObjectTypeQuery Enum") false (`|MakeArray` self :!type "Actor Object Reference")))
  (bind _returnvalue_3 (`NiagaraFunctionLibrary.SpawnSystemAtLocation` "/Game/Particle/LASER.LASER" _returnvalue))
  (`NiagaraComponent.SetVariableVec3` _returnvalue_3 "ABS" _returnvalue_2)
  (for _array_element _outhits
    (`GameplayStatics.ApplyDamage` (`.HitActor` (`GameplayStatics.BreakHitResult` _array_element)) (`.GunDamage_47_C93BDACD4F89739426214C8D7AEABABB` (break `/Game/AircraftData/AircraftDataStructure` (`self.AircraftData`))) (`GameplayStatics.GetPlayerControllerFromID` 0) ParentPlayer "/Game/Blueprints/DamageType/PlayerDamage.PlayerDamage_C")))

(fn `UserConstructionScript`
  (`parent.UserConstructionScript`))